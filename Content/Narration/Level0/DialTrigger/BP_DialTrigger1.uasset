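; BP_DialTrigger1 is a one-shot narration trigger volume that shows up to four dialogue lines to the player character.
; On box overlap, parallel delayed branches fetch lines by index from the first WD_Dialogue widget and fill its four display slots at half-second intervals.
; When the character leaves, it clears all four slots and destroys itself.
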(event `self.Box.OnComponentBeginOverlap`
  (params (OverlappedComponent :type "PrimitiveComponent Object Reference") (OtherActor :type "Actor Object Reference") (OtherComp :type "PrimitiveComponent Object Reference") (OtherBodyIndex :type Integer) (bFromSweep :type Boolean) (SweepResult :type "HitResult Structure (by ref)"))
  (cast `/Game/ThirdPerson/Blueprints/BP_ThirdPersonCharacter` OtherActor)
  (`|ExecutionSequence`
    (:`then_0`
      (bind _foundwidgets (`WidgetBlueprintLibrary.GetAllWidgetsOfClass` "/Game/UI/WD_Dialogue.WD_Dialogue_C"))
      (bind _output (`|GetArrayItem` _foundwidgets))
      (bind (_out_row_id _output_get) (`/Game/UI/WD_Dialogue.GetDialLine` _output (`self.Index1`)))
      (set `/Game/UI/WD_Dialogue.DialToDisplay` (`KismetTextLibrary.Conv_StringToText` (`KismetTextLibrary.Conv_TextToString` _output_get)) _output))
    (:`then_1`
      (bind _foundwidgets_2 (`WidgetBlueprintLibrary.GetAllWidgetsOfClass` "/Game/UI/WD_Dialogue.WD_Dialogue_C"))
      (`KismetSystemLibrary.Delay` 0.5)
      (bind _output_2 (`|GetArrayItem` _foundwidgets_2))
      (bind (_out_row_id_2 _output_get_2) (`/Game/UI/WD_Dialogue.GetDialLine` _output_2 (`self.Index2`)))
      (set `/Game/UI/WD_Dialogue.DialToDisplay2` (`KismetTextLibrary.Conv_StringToText` (`KismetTextLibrary.Conv_TextToString` _output_get_2)) _output_2))
    (:`then_2`
      (bind _foundwidgets_3 (`WidgetBlueprintLibrary.GetAllWidgetsOfClass` "/Game/UI/WD_Dialogue.WD_Dialogue_C"))
      (`KismetSystemLibrary.Delay` 1.0)
      (bind _output_3 (`|GetArrayItem` _foundwidgets_3))
      (bind (_out_row_id_3 _output_get_3) (`/Game/UI/WD_Dialogue.GetDialLine` _output_3 (`self.Index3`)))
      (set `/Game/UI/WD_Dialogue.DialToDisplay3` (`KismetTextLibrary.Conv_StringToText` (`KismetTextLibrary.Conv_TextToString` _output_get_3)) _output_3))
    (:`then_3`
      (bind _foundwidgets_4 (`WidgetBlueprintLibrary.GetAllWidgetsOfClass` "/Game/UI/WD_Dialogue.WD_Dialogue_C"))
      (`KismetSystemLibrary.Delay` 1.5)
      (bind _output_4 (`|GetArrayItem` _foundwidgets_4))
      (bind (_out_row_id_4 _output_get_4) (`/Game/UI/WD_Dialogue.GetDialLine` _output_4 (`self.Index4`)))
      (set `/Game/UI/WD_Dialogue.DialToDisplay4` (`KismetTextLibrary.Conv_StringToText` (`KismetTextLibrary.Conv_TextToString` _output_get_4)) _output_4))))

(event `self.Box.OnComponentEndOverlap`
  (params (OverlappedComponent :type "PrimitiveComponent Object Reference") (OtherActor :type "Actor Object Reference") (OtherComp :type "PrimitiveComponent Object Reference") (OtherBodyIndex :type Integer))
  (cast `/Game/ThirdPerson/Blueprints/BP_ThirdPersonCharacter` OtherActor)
  (bind _foundwidgets (`WidgetBlueprintLibrary.GetAllWidgetsOfClass` "/Game/UI/WD_Dialogue.WD_Dialogue_C"))
  (bind _output (`|GetArrayItem` _foundwidgets))
  (set `/Game/UI/WD_Dialogue.DialToDisplay` "" _output)
  (set `/Game/UI/WD_Dialogue.DialToDisplay2` "" _output)
  (set `/Game/UI/WD_Dialogue.DialToDisplay3` "" _output)
  (set `/Game/UI/WD_Dialogue.DialToDisplay4` "" _output)
  (`self.K2_DestroyActor`))

(fn `UserConstructionScript`)