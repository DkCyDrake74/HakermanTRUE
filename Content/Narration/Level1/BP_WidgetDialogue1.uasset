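; Level 1 narration actor that shows dialogue lines in a TextRender component, one per StartDial event.
; StartDial reads the row at CurrentIndex from DataTable_Dialog1, formats it as "id:Dialog" text, displays it, then increments the index.
; Rows follow the table's row-name order, and the index has no bounds check or reset here.
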(event `StartDial`
  (bind _returnvalue (`self.GetDataTable`))
  (`TextRenderComponent.K2_SetText` (`self.TextRender`) _returnvalue)
  (`self.IncreaseIndex`))

(event `self.ReceiveBeginPlay`)

(fn `GetDataTable`
  (returns (ReturnValue :type Text))
  (bind _outrownames (`DataTableFunctionLibrary.GetDataTableRowNames` "/Game/Narration/Level1/DataTable_Dialog1.DataTable_Dialog1"))
  (bind _returnvalue (`|GetDataTableRow` "/Game/Narration/Level1/DataTable_Dialog1.DataTable_Dialog1" (`|GetArrayItem` _outrownames (`self.CurrentIndex`)))
    (:`then`
      (return (`KismetTextLibrary.Conv_StringToText` (`KismetStringLibrary.Concat_StrStr` (break `/Game/Narration/Level1/Struct_Dialog1` _returnvalue) " : " (`KismetTextLibrary.Conv_TextToString` (`.Dialog_5_30EC4FEC437DB858DDC4CFBB7FF2E175` (break `/Game/Narration/Level1/Struct_Dialog1` _returnvalue)))))))))

(fn `IncreaseIndex`
  (set `self.CurrentIndex` (+ (`self.CurrentIndex`) 1)))

(fn `UserConstructionScript`)