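; Test guard AI that wanders and gets lured to triggered printers or photocopiers.
; A self-repeating Walk event moves it to random reachable points every ten seconds.
; Tick polls two trigger flags, photocopier first, sending the guard to that device, then after its trigger time clearing the flag and resuming wandering.
; Helper functions raise a capped alert level and apprehend the player by destroying the character, though neither is called here.
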(event `ImprimanteIsTrigger`
  (bind _returnvalue (`GameplayStatics.GetActorOfClass` "/Game/Blueprints/Diversion/Imprimantes/BP_Imprimantes.BP_Imprimantes_C"))
  (`AIBlueprintHelperLibrary.SimpleMoveToActor` (`self.GetController`) _returnvalue)
  (`KismetSystemLibrary.Delay` (`/Game/Blueprints/Diversion/Imprimantes/BP_Imprimantes.TriggerTimePrinter` _returnvalue))
  (set `self.ImprimanteIsTrigger?` false)
  (`self.Walk`))

(event `PhotocopieurIsTrigger`
  (bind _returnvalue (`GameplayStatics.GetActorOfClass` "/Game/Blueprints/Diversion/Imprimantes/BP_Photocopier.BP_Photocopier_C"))
  (`|AIMoveTo` self (`/Game/Blueprints/Diversion/Imprimantes/BP_Photocopier.Position` _returnvalue) null
    (:`OnSuccess`
      (`KismetSystemLibrary.Delay` (`/Game/Blueprints/Diversion/Imprimantes/BP_Photocopier.TriggerTime` _returnvalue))
      (set `self.PhotocopieurIsTrigger?` false)
      (`self.Walk`))))

(event `Walk`
  (`|AIMoveTo` self (`NavigationSystemV1.K2_GetRandomReachablePointInRadius` (`self.K2_GetActorLocation`) 1000.0 null null) null
    (:`then`
      (`KismetSystemLibrary.Delay` 10.0)
      (`self.Walk`))))

(event `self.ReceiveBeginPlay`
  (`KismetSystemLibrary.Delay` 1.0)
  (`self.Walk`))

(event `self.ReceiveTick`
  (params (DeltaSeconds :type "Float (single-precision)"))
  (if (`self.PhotocopieurIsTrigger?`)
    (`self.PhotocopieurIsTrigger`)
    (elif (`self.ImprimanteIsTrigger?`)
      (`self.ImprimanteIsTrigger`))))

(fn `Apprehend`
  (bind _asbp_third_person_character (cast `/Game/ThirdPerson/Blueprints/BP_ThirdPersonCharacter` (`GameplayStatics.GetPlayerCharacter` 0)))
  (`self.K2_DestroyActor` _asbp_third_person_character))

(fn `IncreaseAlertLevel`
  (if (< (`self.AlertLevel`) (`self.MaxAlertLevel`))
    (set `self.AlertLevel` (+ 1 (`self.AlertLevel`)))))

(fn `UserConstructionScript`)