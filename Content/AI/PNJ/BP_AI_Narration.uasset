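; BP_AI_Narration is an NPC AI Blueprint that tracks an alert level and can apprehend the player.
; IncreaseAlertLevel raises AlertLevel one step at a time up to MaxAlertLevel.
; Apprehend casts player 0's character to BP_ThirdPersonCharacter and destroys that actor.
; Neither function is called within this Blueprint, and no logic here links the alert level to apprehension.
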(fn `Apprehend`
  (bind _asbp_third_person_character (cast `/Game/ThirdPerson/Blueprints/BP_ThirdPersonCharacter` (`GameplayStatics.GetPlayerCharacter` 0)))
  (`self.K2_DestroyActor` _asbp_third_person_character))

(fn `IncreaseAlertLevel`
  (if (< (`self.AlertLevel`) (`self.MaxAlertLevel`))
    (set `self.AlertLevel` (+ 1 (`self.AlertLevel`)))))

(fn `UserConstructionScript`)