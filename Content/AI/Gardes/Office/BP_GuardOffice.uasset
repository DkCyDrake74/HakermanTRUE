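; BP_GuardOffice is an office guard that watches for pawns and alerts the Level 2 guard squad when suspicious.
; PawnSensing sightings raise Suspicion in small steps up to a cap, and Tick checks it against a fixed threshold.
; At the threshold, TransferPlayerPosition calls OnAlertLevel2 on every "Squad"-tagged guard, repeating each tick without passing a position.
; LightEvent clears LightClose and disables sensing updates.
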(event `TransferPlayerPosition`
  (bind _outactors (`GameplayStatics.GetAllActorsOfClassWithTag` "/Game/AI/Gardes/Level2/GardesRandom/BP_AI_gardes_Level_2.BP_AI_gardes_Level_2_C" "Squad"))
  (for _array_element _outactors
    (`/Game/AI/Gardes/Level2/GardesRandom/BP_AI_gardes_Level_2.OnAlertLevel2` _array_element)))

(event `VerifSuspition`
  (if (>= (`self.Suspicion`) 5.0)
    (`self.TransferPlayerPosition`)))

(event `IncreaseSuspition`
  (if (<= (`self.Suspicion`) (`self.SuspicionMax`))
    (set `self.Suspicion` (+ (`self.Suspicion`) 0.1))))

(event `self.PawnSensing.OnSeePawn`
  (params (Pawn :type "Pawn Object Reference"))
  (`self.IncreaseSuspition`))

(event `self.ReceiveTick`
  (params (DeltaSeconds :type "Float (single-precision)"))
  (`self.VerifSuspition`))

(event `LightEvent`
  (set `self.LightClose` false)
  (`PawnSensingComponent.SetSensingUpdatesEnabled` (`self.PawnSensing`) false))

(fn `UserConstructionScript`)