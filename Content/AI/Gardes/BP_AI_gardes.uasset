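; Guard AI character that wanders to random reachable points and hunts the player through escalating alert levels.
; Each PawnSensing sighting raises a capped alert level that never decreases, and higher alerts shorten the sensing interval.
; First alert pauses, then moves to the player's position; maximum alert chases faster and destroys the player on arrival.
; A failed chase slows the guard and sends it to the player's location at that moment.
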(event `OnAlertLevel1`
  (bind _output_get (set `self.SensingInterval` 3.0))
  (`PawnSensingComponent.SetSensingInterval` (`self.PawnSensing`) _output_get)
  (`MovementComponent.StopMovementImmediately` (`self.CharacterMovement`))
  (`KismetSystemLibrary.Delay` 2.0)
  (bind _asbp_third_person_character (cast `/Game/ThirdPerson/Blueprints/BP_ThirdPersonCharacter` (`GameplayStatics.GetPlayerCharacter` 0)))
  (bind _output_get_2 (set `self.PlayerPosition?` (`self.K2_GetActorLocation` _asbp_third_person_character)))
  (`|AIMoveTo` self _output_get_2 null
    (:`OnSuccess`
      (`KismetSystemLibrary.PrintString` "Arriver a la position"))))

(event `OnAlertLevel2`
  (bind _charactermovement (`self.CharacterMovement`))
  (bind _output_get (set `self.SensingInterval` 1.0))
  (`PawnSensingComponent.SetSensingInterval` (`self.PawnSensing`) _output_get)
  (bind _returnvalue (`self.K2_GetActorLocation` (stale `self.PawnSensing.OnSeePawn` _asbp_third_person_character)))
  (`|AIMoveTo` self _returnvalue (stale `self.PawnSensing.OnSeePawn` _asbp_third_person_character)
    (:`then`
      (`KismetSystemLibrary.PrintText` "Alert Max" true true (struct :`R` 0.677083 :`B` 0.014692 :`A` 1.0) 0.5)
      (set `CharacterMovementComponent.MaxWalkSpeed` 300.0 _charactermovement))
    (:`OnSuccess`
      (`self.Apprehend`))
    (:`OnFail`
      (`KismetSystemLibrary.PrintString` "Break LOS" true true (struct :`G` 0.66 :`B` 1.0 :`A` 1.0) 0.5)
      (set `CharacterMovementComponent.MaxWalkSpeed` 180.0 _charactermovement)
      (bind _output_get_2 (set `self.LastKnowPawnPosition` _returnvalue))
      (`KismetSystemLibrary.PrintString` (`KismetStringLibrary.Conv_VectorToString` _output_get_2))
      (`|AIMoveTo` self _output_get_2 null))))

(event `self.PawnSensing.OnSeePawn`
  (params (Pawn :type "Pawn Object Reference"))
  (bind _asbp_third_person_character (cast `/Game/ThirdPerson/Blueprints/BP_ThirdPersonCharacter` Pawn))
  (`self.IncreaseAlertLevel`)
  (if (== (`self.AlertLevel`) 1)
    (`self.OnAlertLevel1`)
    (elif (== (`self.MaxAlertLevel`) (`self.AlertLevel`))
      (`self.OnAlertLevel2`)
      (else
        (`self.Walk`)))))

(event `Walk`
  (`|AIMoveTo` self (`NavigationSystemV1.K2_GetRandomReachablePointInRadius` (`self.K2_GetActorLocation`) 1000.0 null null) null
    (:`then`
      (`KismetSystemLibrary.Delay` 10.0)
      (`self.Walk`))))

(event `self.ReceiveBeginPlay`
  (`KismetSystemLibrary.Delay` 1.0)
  (`self.Walk`))

(event `self.ReceiveTick`
  (params (DeltaSeconds :type "Float (single-precision)"))
  (`KismetSystemLibrary.PrintString` (`KismetStringLibrary.Conv_IntToString` (`self.AlertLevel`)) true true (struct :`R` 0.012149 :`G` 1.0 :`A` 1.0) 0.01)
  (`KismetSystemLibrary.PrintString` (`KismetStringLibrary.Conv_DoubleToString` (`self.SensingInterval`)) true true (struct :`G` 0.347514 :`B` 1.0 :`A` 1.0) 0.01)
  (`KismetSystemLibrary.PrintString` (`KismetStringLibrary.Conv_VectorToString` (`self.K2_GetActorLocation`)) true true (struct :`R` 0.651042 :`B` 0.010906 :`A` 1.0) 0.01))

(fn `Apprehend`
  (bind _asbp_third_person_character (cast `/Game/ThirdPerson/Blueprints/BP_ThirdPersonCharacter` (`GameplayStatics.GetPlayerCharacter` 0)))
  (`self.K2_DestroyActor` _asbp_third_person_character))

(fn `IncreaseAlertLevel`
  (if (< (`self.AlertLevel`) (`self.MaxAlertLevel`))
    (set `self.AlertLevel` (+ 1 (`self.AlertLevel`)))))

(fn `UserConstructionScript`)