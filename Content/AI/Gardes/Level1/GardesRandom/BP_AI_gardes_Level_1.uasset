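; Level 1 guard AI that patrols randomly around its spawn point and hunts the player in a stealth game.
; Pawn sensing builds suspicion, checked on Tick to trigger two alert levels: investigate, then arm and approach.
; A forward sphere trace jumps to level 2; a rear trigger catches non-crouched players.
; Contact plays an attack and reloads the map after a delay, while triggered printers in range divert the guard.
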(event `VerifSuspition`
  ;[0.1006 1 0] Verif susption for increase alert level
  (`|ExecutionSequence`
    (:`then_0`
      (if (>= (`self.Suspition`) 2.5)
        (`self.OnAlertLevel1`)))
    (:`then_1`
      (if (>= (`self.Suspition`) 5.0)
        (`self.OnAlertLevel2`)))))

(event `IncreaseSuspition`
  ;[0.145 1 0] Increase suspition
  (if (<= (`self.Suspition`) (`self.SuspitionMax`))
    (set `self.Suspition` (+ (`self.Suspition`) 0.1))))

(event `SpawnWeapon`
  (`/Engine/EditorBlueprintResources/StandardMacros.DoOnce` false
    (:`Completed`
      (bind _returnvalue (`|SpawnActorFromClass` "/Game/AI/Weapon/BP_Weapon.BP_Weapon_C" (`SceneComponent.GetSocketTransform` (`self.Mesh`) "WeaponSocket" "RTS_World") "Undefined" "OverrideRootScale" null null))
      (`self.K2_AttachToComponent` _returnvalue (`self.Mesh`) "WeaponSocket" "SnapToTarget" "SnapToTarget" "SnapToTarget" true))))

(event `OnAlertLevel1`
  ;[1 0.4558 0] Alert level 1
  (`/Engine/EditorBlueprintResources/StandardMacros.DoOnce` false
    (:`Completed`
      (bind _asbp_third_person_character (cast `/Game/ThirdPerson/Blueprints/BP_ThirdPersonCharacter` (`GameplayStatics.GetPlayerCharacter` 0)))
      (bind _output_get (set `self.PlayerPosition?` (`self.K2_GetActorLocation` _asbp_third_person_character)))
      (`|AIMoveTo` self _output_get null 20.0
        (:`OnSuccess`
          (`KismetSystemLibrary.Delay` (`KismetMathLibrary.RandomFloatInRange` 5.0 10.0))
          (`self.Walk`))
        (:`OnFail`
          (`self.Walk`))))))

(event `MoveToInitPos`
  ;[0.04174 1 0] Move to the initial position
  (`|AIMoveTo` self (`self.AIInitPosition`) null))

(event `OnAlertLevel2`
  (bind _returnvalue (`GameplayStatics.GetPlayerCharacter` 0))
  (bind _charactermovement (`self.CharacterMovement`))
  ;[1 0.01854 0] Alert level 2
  (`self.SpawnWeapon`)
  (cast `/Game/ThirdPerson/Blueprints/BP_ThirdPersonCharacter` _returnvalue)
  (`|AIMoveTo` self (`self.K2_GetActorLocation` _returnvalue) null
    (:`then`
      (set `CharacterMovementComponent.MaxWalkSpeed` 250.0 _charactermovement))
    (:`OnFail`
      (set `CharacterMovementComponent.MaxWalkSpeed` 180.0 _charactermovement)
      (`self.Walk`))))

(event `RaycastFront`
  (bind _aipos (`self.AIPos`))
  ;[0.6719 0.00802 0] Raycast front to trigger the alert 2
  (bind _outhit (`KismetSystemLibrary.SphereTraceSingleByProfile` _aipos (+ _aipos (* (`self.GetActorForwardVector`) 400)) 90.0 "Pawn"))
  (if (== (`GameplayStatics.GetObjectClass` (`.HitActor` (`GameplayStatics.BreakHitResult` _outhit))) "/Game/ThirdPerson/Blueprints/BP_ThirdPersonCharacter.BP_ThirdPersonCharacter_C")
    (`AudioComponent.Play` (`self.Alarm`) 0.0)
    (`self.OnAlertLevel2`)))

(event `self.ReceiveBeginPlay`
  ;[0 0.2482 1] Set initial position + ref to the anim blueprint
  (set `self.AIInitPosition` (`self.K2_GetActorLocation`))
  (bind _asanim_blueprint_garde_level_1 (cast `/Game/AI/Gardes/Animation/Level1/AnimBlueprint_GardeLevel1` (`SkeletalMeshComponent.GetAnimInstance` (`self.Mesh`))))
  (set `self.As Anim Blueprint Garde Level 1` _asanim_blueprint_garde_level_1)
  (`KismetSystemLibrary.Delay` 1.0)
  (`self.Walk`))

(event `self.PawnSensing.OnSeePawn`
  (params (Pawn :type "Pawn Object Reference"))
  ;[1 0.891 0] Pawn Sensing
  (`self.IncreaseSuspition`))

(event `self.TriggerColliderBack.OnComponentBeginOverlap`
  (params (OverlappedComponent :type "PrimitiveComponent Object Reference") (OtherActor :type "Actor Object Reference") (OtherComp :type "PrimitiveComponent Object Reference") (OtherBodyIndex :type Integer) (bFromSweep :type Boolean) (SweepResult :type "HitResult Structure (by ref)"))
  ;[1 0.3756 0] Trigger guard back
  (bind _asbp_third_person_character (cast `/Game/ThirdPerson/Blueprints/BP_ThirdPersonCharacter` OtherActor))
  (if (not (`/Game/ThirdPerson/Blueprints/BP_ThirdPersonCharacter.isCrouch?` _asbp_third_person_character))
    (`AudioComponent.Play` (`self.Trigger`) 0.0)
    (`KismetSystemLibrary.Delay` 2.0)
    (`self.OnAlertLevel1`)))

(event `Walk`
  (bind _as_anim_blueprint_garde_level_1 (`self.As Anim Blueprint Garde Level 1`))
  ;[0.02952 1 0] Walk Semi Random
  (`|AIMoveTo` self (`NavigationSystemV1.K2_GetRandomReachablePointInRadius` (`self.AIInitPosition`) (`KismetMathLibrary.RandomFloatInRange` (`self.RandomRadiusMin`) (`self.RandomRadiusMax`)) null null) null
    (:`OnSuccess`
      (set `/Game/AI/Gardes/Animation/Level1/AnimBlueprint_GardeLevel1.Is Looking` true _as_anim_blueprint_garde_level_1)
      (`KismetSystemLibrary.Delay` (`KismetMathLibrary.RandomFloatInRange` (`self.RandomDelayMin`) (`self.RandomDelayMax`)))
      (set `/Game/AI/Gardes/Animation/Level1/AnimBlueprint_GardeLevel1.Is Looking` false _as_anim_blueprint_garde_level_1)
      (`|AIMoveTo` self (`self.AIInitPosition`) null
        (:`OnSuccess`
          (`self.Walk`))
        (:`OnFail`
          (`self.Walk`))))
    (:`OnFail`
      (`|AIMoveTo` self (`self.AIInitPosition`) null
        (:`OnSuccess`
          (`self.Walk`))
        (:`OnFail`
          (`self.Walk`))))))

(event `self.TriggerColliderOnGuard.OnComponentBeginOverlap`
  (params (OverlappedComponent :type "PrimitiveComponent Object Reference") (OtherActor :type "Actor Object Reference") (OtherComp :type "PrimitiveComponent Object Reference") (OtherBodyIndex :type Integer) (bFromSweep :type Boolean) (SweepResult :type "HitResult Structure (by ref)"))
  (bind _as_anim_blueprint_garde_level_1 (`self.As Anim Blueprint Garde Level 1`))
  ;[1 0.3943 0] Trigger guard
  (bind _asbp_third_person_character (cast `/Game/ThirdPerson/Blueprints/BP_ThirdPersonCharacter` OtherActor))
  (cast `/Game/ThirdPerson/Blueprints/BP_ThirdPersonGameMode` (`GameplayStatics.GetGameMode`))
  (set `/Game/AI/Gardes/Animation/Level1/AnimBlueprint_GardeLevel1.Is attack` true _as_anim_blueprint_garde_level_1)
  (`self.MoveToInitPos`)
  (`KismetSystemLibrary.Delay` 8.0)
  (`GameplayStatics.OpenLevel` "ThirdPersonMap")
  (set `/Game/AI/Gardes/Animation/Level1/AnimBlueprint_GardeLevel1.Is attack` false _as_anim_blueprint_garde_level_1)
  (set `/Game/ThirdPerson/Blueprints/BP_ThirdPersonCharacter.IsAttacked` false _asbp_third_person_character))

(event `self.ReceiveTick`
  (params (DeltaSeconds :type "Float (single-precision)"))
  ;[0 0.04742 1] Event tick
  (`|ExecutionSequence`
    (:`then_0`
      (set `self.AIPos` (`self.K2_GetActorLocation`))
      (if (`/Game/AI/Gardes/Animation/Level1/AnimBlueprint_GardeLevel1.Is attack` (`self.As Anim Blueprint Garde Level 1`))
        (`MovementComponent.StopMovementImmediately` (`self.CharacterMovement`)))
      (`self.RaycastFront`)
      (`self.VerifSuspition`))
    (:`then_1`
      (if (`self.printerIsInRange`)
        (if (`self.ImprimanteIsTrigger`)
          (bind _returnvalue (`GameplayStatics.GetActorOfClass` "/Game/Blueprints/Diversion/Level1/BP_Imprimantes_Level_1.BP_Imprimantes_Level_1_C"))
          (`|AIMoveTo` self (`/Game/Blueprints/Diversion/Level1/BP_Imprimantes_Level_1.PositionPrinter` _returnvalue) null 30.0
            (:`OnSuccess`
              (set `self.ImprimanteIsTrigger` false)
              (`KismetSystemLibrary.Delay` (`/Game/Blueprints/Diversion/Level1/BP_Imprimantes_Level_1.TriggerTimePrinter` _returnvalue))
              (`self.MoveToInitPos`)
              (`self.Walk`))))))))

(fn `Apprehend`
  (bind _asbp_third_person_character (cast `/Game/ThirdPerson/Blueprints/BP_ThirdPersonCharacter` (`GameplayStatics.GetPlayerCharacter` 0)))
  (`self.K2_DestroyActor` _asbp_third_person_character))

(fn `UserConstructionScript`)