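; Office guard AI for Level 2 that patrols a looping chain of six waypoint actors with random pauses.
; PawnSensing sightings raise an alert level: the first stops the guard and walks it to the player's position, the maximum starts a faster chase.
; A successful chase destroys the player; a failed one slows the guard and moves toward the player's current position.
; A Tick-polled flag diverts it to ringing phones before patrol resumes.
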(event `OnAlertLevel1`
  (bind _output_get (set `self.SensingInterval` 3.0))
  (`PawnSensingComponent.SetSensingInterval` (`self.PawnSensing`) _output_get)
  (`MovementComponent.StopMovementImmediately` (`self.CharacterMovement`))
  (`KismetSystemLibrary.Delay` 2.0)
  (bind _asbp_third_person_character (cast `/Game/ThirdPerson/Blueprints/BP_ThirdPersonCharacter` (`GameplayStatics.GetPlayerCharacter` 0)))
  (bind _output_get_2 (set `self.PlayerPosition?` (`self.K2_GetActorLocation` _asbp_third_person_character)))
  (`|AIMoveTo` self _output_get_2 null
    (:`OnSuccess`
      (`KismetSystemLibrary.PrintString` "Arriver a la position"))))

(event `OnAlertLevel2`
  (bind _charactermovement (`self.CharacterMovement`))
  (bind _output_get (set `self.SensingInterval` 1.0))
  (`PawnSensingComponent.SetSensingInterval` (`self.PawnSensing`) _output_get)
  (bind _returnvalue (`self.K2_GetActorLocation` (stale `self.PawnSensing.OnSeePawn` _asbp_third_person_character)))
  (`|AIMoveTo` self _returnvalue (stale `self.PawnSensing.OnSeePawn` _asbp_third_person_character)
    (:`then`
      (`KismetSystemLibrary.PrintText` "Alert Max" true true (struct :`R` 0.677083 :`B` 0.014692 :`A` 1.0) 0.5)
      (set `CharacterMovementComponent.MaxWalkSpeed` 250.0 _charactermovement))
    (:`OnSuccess`
      (`self.Apprehend`))
    (:`OnFail`
      (`KismetSystemLibrary.PrintString` "Break LOS" true true (struct :`G` 0.66 :`B` 1.0 :`A` 1.0) 0.5)
      (set `CharacterMovementComponent.MaxWalkSpeed` 180.0 _charactermovement)
      (bind _output_get_2 (set `self.LastKnowPawnPosition` _returnvalue))
      (`KismetSystemLibrary.PrintString` (`KismetStringLibrary.Conv_VectorToString` _output_get_2))
      (`|AIMoveTo` self _output_get_2 null))))

(event `self.PawnSensing.OnSeePawn`
  (params (Pawn :type "Pawn Object Reference"))
  (bind _asbp_third_person_character (cast `/Game/ThirdPerson/Blueprints/BP_ThirdPersonCharacter` Pawn))
  (`self.IncreaseAlertLevel`)
  (if (== (`self.AlertLevel`) 1)
    (`self.OnAlertLevel1`)
    (elif (== (`self.MaxAlertLevel`) (`self.AlertLevel`))
      (`self.OnAlertLevel2`)
      (else
        (`self.Walk`)))))

(event `self.ReceiveBeginPlay`
  (`KismetSystemLibrary.Delay` 1.0)
  (`self.Walk`))

(event `PhoneIsTrigger`
  (bind _outactors (`GameplayStatics.GetAllActorsOfClass` "/Game/Blueprints/Diversion/Phone/BP_Diversion_Phone.BP_Diversion_Phone_C"))
  (for _array_element _outactors
    (`|AIMoveTo` self (`/Game/Blueprints/Diversion/Phone/BP_Diversion_Phone.PositionPhone` _array_element) null
      (:`OnSuccess`
        (`KismetSystemLibrary.Delay` (`/Game/Blueprints/Diversion/Phone/BP_Diversion_Phone.TriggerTimePhone` _array_element))
        (set `self.PhoneIsTrigger?` false)
        (bind _returnvalue (`GameplayStatics.GetActorOfClass` "/Game/Blueprints/Diversion/Phone/BP_Diversion_Phone.BP_Diversion_Phone_C"))
        (set `/Game/Blueprints/Diversion/Phone/BP_Diversion_Phone.alarmOn` false _returnvalue)
        (`self.Walk`)))))

(event `self.ReceiveTick`
  (params (DeltaSeconds :type "Float (single-precision)"))
  (if (`self.PhoneIsTrigger?`)
    (`self.PhoneIsTrigger`)))

(event `Walk`
  ;[0.001953 0 1] Walk Waypoints
  (bind _returnvalue (`GameplayStatics.GetActorOfClass` "/Game/AI/Gardes/Level2/Gardes_Office/Waypoints/Waypoints.Waypoints_C"))
  (`|AIMoveTo` self (0.0 0.0 0.0) _returnvalue
    (:`OnSuccess`
      (`KismetSystemLibrary.Delay` (`KismetMathLibrary.RandomFloatInRange` 3.0 7.0))
      (bind _returnvalue_2 (`GameplayStatics.GetActorOfClass` "/Game/AI/Gardes/Level2/Gardes_Office/Waypoints/Waypoints1.Waypoints1_C"))
      (`|AIMoveTo` self (0.0 0.0 0.0) _returnvalue_2
        (:`OnSuccess`
          (`KismetSystemLibrary.Delay` (`KismetMathLibrary.RandomFloatInRange` 3.0 7.0))
          (bind _returnvalue_3 (`GameplayStatics.GetActorOfClass` "/Game/AI/Gardes/Level2/Gardes_Office/Waypoints/Waypoints2.Waypoints2_C"))
          (`|AIMoveTo` self (0.0 0.0 0.0) _returnvalue_3
            (:`OnSuccess`
              (`KismetSystemLibrary.Delay` (`KismetMathLibrary.RandomFloatInRange` 3.0 7.0))
              (bind _returnvalue_4 (`GameplayStatics.GetActorOfClass` "/Game/AI/Gardes/Level2/Gardes_Office/Waypoints/Waypoints3.Waypoints3_C"))
              (`|AIMoveTo` self (0.0 0.0 0.0) _returnvalue_4
                (:`OnSuccess`
                  (`KismetSystemLibrary.Delay` (`KismetMathLibrary.RandomFloatInRange` 3.0 7.0))
                  (bind _returnvalue_5 (`GameplayStatics.GetActorOfClass` "/Game/AI/Gardes/Level2/Gardes_Office/Waypoints/Waypoints4.Waypoints4_C"))
                  (`|AIMoveTo` self (0.0 0.0 0.0) _returnvalue_5
                    (:`OnSuccess`
                      (`KismetSystemLibrary.Delay` (`KismetMathLibrary.RandomFloatInRange` 3.0 7.0))
                      (bind _returnvalue_6 (`GameplayStatics.GetActorOfClass` "/Game/AI/Gardes/Level2/Gardes_Office/Waypoints/Waypoints5.Waypoints5_C"))
                      (`|AIMoveTo` self (0.0 0.0 0.0) _returnvalue_6
                        (:`OnSuccess`
                          (`KismetSystemLibrary.Delay` (`KismetMathLibrary.RandomFloatInRange` 3.0 7.0))
                          (`self.Walk`))))))))))))))

(fn `Apprehend`
  (bind _asbp_third_person_character (cast `/Game/ThirdPerson/Blueprints/BP_ThirdPersonCharacter` (`GameplayStatics.GetPlayerCharacter` 0)))
  (`self.K2_DestroyActor` _asbp_third_person_character))

(fn `IncreaseAlertLevel`
  (if (< (`self.AlertLevel`) (`self.MaxAlertLevel`))
    (set `self.AlertLevel` (+ 1 (`self.AlertLevel`)))))

(fn `UserConstructionScript`)