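; Guard AI that wanders randomly around its spawn point, detects the player and catches them on contact, triggering a respawn.
; PawnSensing sightings build suspicion, checked each Tick against two alert thresholds: a one-time investigation of the player's position, then a faster pursuit.
; A per-frame forward sphere trace jumps straight to pursuit with an alarm.
; A rear trigger starts a delayed investigation when the player is not crouched.
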(event `VerifSuspition`
  (`|ExecutionSequence`
    (:`then_0`
      (if (>= (`self.Suspition`) 2.5)
        (`self.OnAlertLevel1`)))
    (:`then_1`
      (if (>= (`self.Suspition`) 5.0)
        (`self.OnAlertLevel2`)))))

(event `IncreaseSuspition`
  (if (<= (`self.Suspition`) (`self.SuspitionMax`))
    (set `self.Suspition` (+ (`self.Suspition`) 0.1))))

(event `OnAlertLevel1`
  (`/Engine/EditorBlueprintResources/StandardMacros.DoOnce` false
    (:`Completed`
      (bind _asbp_third_person_character (cast `/Game/ThirdPerson/Blueprints/BP_ThirdPersonCharacter` (`GameplayStatics.GetPlayerCharacter` 0)))
      (bind _output_get (set `self.PlayerPosition?` (`self.K2_GetActorLocation` _asbp_third_person_character)))
      (`|AIMoveTo` self _output_get null 20.0
        (:`OnSuccess`
          (`KismetSystemLibrary.Delay` (`KismetMathLibrary.RandomFloatInRange` 5.0 10.0))
          (`self.Walk`))
        (:`OnFail`
          (`self.Walk`))))))

(event `OnAlertLevel2`
  (bind _returnvalue (`GameplayStatics.GetPlayerCharacter` 0))
  (bind _charactermovement (`self.CharacterMovement`))
  (cast `/Game/ThirdPerson/Blueprints/BP_ThirdPersonCharacter` _returnvalue)
  (`|AIMoveTo` self (`self.K2_GetActorLocation` _returnvalue) null
    (:`then`
      (set `CharacterMovementComponent.MaxWalkSpeed` 250.0 _charactermovement))
    (:`OnFail`
      (set `CharacterMovementComponent.MaxWalkSpeed` 180.0 _charactermovement)
      (`self.Walk`))))

(event `RaycastFront`
  (bind _aipos (`self.AIPos`))
  (bind _outhit (`KismetSystemLibrary.SphereTraceSingleByProfile` _aipos (+ _aipos (* (`self.GetActorForwardVector`) 400)) 90.0 "Pawn"))
  (if (== (`GameplayStatics.GetObjectClass` (`.HitActor` (`GameplayStatics.BreakHitResult` _outhit))) "/Game/ThirdPerson/Blueprints/BP_ThirdPersonCharacter.BP_ThirdPersonCharacter_C")
    (`AudioComponent.Play` (`self.Alarm`) 0.0)
    (`self.OnAlertLevel2`)))

(event `self.PawnSensing.OnSeePawn`
  (params (Pawn :type "Pawn Object Reference"))
  (`self.IncreaseSuspition`))

(event `self.TriggerColliderBack.OnComponentBeginOverlap`
  (params (OverlappedComponent :type "PrimitiveComponent Object Reference") (OtherActor :type "Actor Object Reference") (OtherComp :type "PrimitiveComponent Object Reference") (OtherBodyIndex :type Integer) (bFromSweep :type Boolean) (SweepResult :type "HitResult Structure (by ref)"))
  (bind _asbp_third_person_character (cast `/Game/ThirdPerson/Blueprints/BP_ThirdPersonCharacter` OtherActor))
  (if (not (`/Game/ThirdPerson/Blueprints/BP_ThirdPersonCharacter.isCrouch?` _asbp_third_person_character))
    (`AudioComponent.Play` (`self.Trigger`) 0.0)
    (`KismetSystemLibrary.Delay` 2.0)
    (`self.OnAlertLevel1`)))

(event `Walk`
  ;[0.02952 1 0] Walk Semi Random
  (`|AIMoveTo` self (`NavigationSystemV1.K2_GetRandomReachablePointInRadius` (`self.AIInitPosition`) (`KismetMathLibrary.RandomFloatInRange` (`self.RandomRadiusMin`) (`self.RandomRadiusMax`)) null null) null
    (:`OnSuccess`
      (`KismetSystemLibrary.Delay` (`KismetMathLibrary.RandomFloatInRange` (`self.RandomDelayMin`) (`self.RandomDelayMax`)))
      (`|AIMoveTo` self (`self.AIInitPosition`) null
        (:`OnSuccess`
          (`self.Walk`))
        (:`OnFail`
          (`self.Walk`))))
    (:`OnFail`
      (`|AIMoveTo` self (`self.AIInitPosition`) null
        (:`OnSuccess`
          (`self.Walk`))
        (:`OnFail`
          (`self.Walk`))))))

(event `self.TriggerColliderOnGuard.OnComponentBeginOverlap`
  (params (OverlappedComponent :type "PrimitiveComponent Object Reference") (OtherActor :type "Actor Object Reference") (OtherComp :type "PrimitiveComponent Object Reference") (OtherBodyIndex :type Integer) (bFromSweep :type Boolean) (SweepResult :type "HitResult Structure (by ref)"))
  (bind _asbp_third_person_character (cast `/Game/ThirdPerson/Blueprints/BP_ThirdPersonCharacter` OtherActor))
  (bind _asbp_third_person_game_mode (cast `/Game/ThirdPerson/Blueprints/BP_ThirdPersonGameMode` (`GameplayStatics.GetGameMode`)))
  (`/Game/ThirdPerson/Blueprints/BP_ThirdPersonGameMode.RespawnPlayer` _asbp_third_person_game_mode)
  (`self.K2_DestroyActor` _asbp_third_person_character))

(event `self.ReceiveTick`
  (params (DeltaSeconds :type "Float (single-precision)"))
  (set `self.AIPos` (`self.K2_GetActorLocation`))
  (`self.RaycastFront`)
  (`self.VerifSuspition`))

(event `self.ReceiveBeginPlay`
  (set `self.AIInitPosition` (`self.K2_GetActorLocation`))
  (`KismetSystemLibrary.Delay` 1.0)
  (`self.Walk`))

(fn `Apprehend`
  (bind _asbp_third_person_character (cast `/Game/ThirdPerson/Blueprints/BP_ThirdPersonCharacter` (`GameplayStatics.GetPlayerCharacter` 0)))
  (`self.K2_DestroyActor` _asbp_third_person_character))

(fn `UserConstructionScript`)