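; Level 2 guard AI that wanders randomly around its spawn point, pausing to look around, and hunts the player.
; Sight, a rear trigger and a front sphere trace feed two alert levels: investigate, then armed run with alarm.
; Touching the player plays a taser game over and reloads the level.
; Tick-polled flags send it to distraction props, while the fusebox event electrocutes it and disables its senses.
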(event `VerifSuspition`
  ;[0.1006 1 0] Verif susption for increase alert level
  (`|ExecutionSequence`
    (:`then_0`
      (if (>= (`self.Suspition`) 1.0)
        (`self.OnAlertLevel1`)))
    (:`then_1`
      (if (>= (`self.Suspition`) 5.0)
        (`self.OnAlertLevel2`)))))

(event `IncreaseSuspition`
  ;[0.145 1 0] Increase suspition
  (if (<= (`self.Suspition`) (`self.SuspitionMax`))
    (set `self.Suspition` (+ (`self.Suspition`) 0.1))))

(event `SpawnWeapon`
  (`/Engine/EditorBlueprintResources/StandardMacros.DoOnce` false
    (:`Completed`
      (bind _returnvalue (`|SpawnActorFromClass` "/Game/AI/Weapon/BP_Weapon.BP_Weapon_C" (`SceneComponent.GetSocketTransform` (`self.Mesh`) "WeaponSocket" "RTS_World") "Undefined" "OverrideRootScale" null null))
      (`self.K2_AttachToComponent` _returnvalue (`self.Mesh`) "WeaponSocket" "SnapToTarget" "SnapToTarget" "SnapToTarget" true))))

(event `OnAlertLevel1`
  (bind _as_anim_blueprint_garde (`self.As Anim Blueprint Garde`))
  (bind _as_anim_blueprint_garde_2 (`self.As Anim Blueprint Garde`))
  (if (not (`/Game/AI/Gardes/Animation/Level2/AnimBlueprint_GardeRandomLevel2.IsElectrocuted` _as_anim_blueprint_garde))
    ;[1 0.4558 0] Alert level 1
    (set `/Game/AI/Gardes/Animation/Level2/AnimBlueprint_GardeRandomLevel2.OnAlert` true _as_anim_blueprint_garde)
    (`/Engine/EditorBlueprintResources/StandardMacros.DoOnce` false
      (:`Completed`
        (`GameplayStatics.PlaySound2D` "/Game/AI/Gardes/Level2/GardesDebut/Audio/Spotted.Spotted" 1.0 1.0 0.0 null null)
        (bind _asbp_third_person_character (cast `/Game/ThirdPerson/Blueprints/BP_ThirdPersonCharacter` (`GameplayStatics.GetPlayerCharacter` 0)))
        (bind _output_get (set `self.PlayerPosition?` (`self.K2_GetActorLocation` _asbp_third_person_character)))
        (`|AIMoveTo` self _output_get null 20.0
          (:`OnSuccess`
            (set `/Game/AI/Gardes/Animation/Level2/AnimBlueprint_GardeRandomLevel2.OnAlertIdle` true (`self.As Anim Blueprint Garde`))
            (`KismetSystemLibrary.Delay` (`KismetMathLibrary.RandomFloatInRange` 5.0 10.0))
            (`self.Walk`)
            (set `/Game/AI/Gardes/Animation/Level2/AnimBlueprint_GardeRandomLevel2.OnAlert` false _as_anim_blueprint_garde_2)
            (set `/Game/AI/Gardes/Animation/Level2/AnimBlueprint_GardeRandomLevel2.OnAlertIdle` false _as_anim_blueprint_garde_2))
          (:`OnFail`
            (`self.Walk`)))))))

(event `MoveToInitPos`
  ;[0.04174 1 0] Move to the initial position
  (`|AIMoveTo` self (`self.AIInitPosition`) null))

(event `OnAlertLevel2`
  (bind _as_anim_blueprint_garde (`self.As Anim Blueprint Garde`))
  (bind _as_anim_blueprint_garde_2 (`self.As Anim Blueprint Garde`))
  (bind _charactermovement (`self.CharacterMovement`))
  (if (not (`/Game/AI/Gardes/Animation/Level2/AnimBlueprint_GardeRandomLevel2.IsElectrocuted` _as_anim_blueprint_garde))
    (set `/Game/AI/Gardes/Animation/Level2/AnimBlueprint_GardeRandomLevel2.OnAlertMax` false _as_anim_blueprint_garde)
    (set `/Game/AI/Gardes/Animation/Level2/AnimBlueprint_GardeRandomLevel2.OnAlertMax` true _as_anim_blueprint_garde)
    (set `self.Suspition` 5.0)
    (`|ExecutionSequence`
      (:`then_0`
        (set `CharacterMovementComponent.MaxWalkSpeed` 300.0 (`self.CharacterMovement`))
        (`self.SpawnWeapon`)
        ;[1 0.01854 0] Alert level 2
        (set `/Game/AI/Gardes/Animation/Level2/AnimBlueprint_GardeRandomLevel2.OnAlert` false _as_anim_blueprint_garde_2)
        (set `/Game/AI/Gardes/Animation/Level2/AnimBlueprint_GardeRandomLevel2.GuardRun` true _as_anim_blueprint_garde_2)
        (bind _asbp_third_person_character (cast `/Game/ThirdPerson/Blueprints/BP_ThirdPersonCharacter` (`GameplayStatics.GetPlayerCharacter` 0)))
        (`|AIMoveTo` self (`self.K2_GetActorLocation` _asbp_third_person_character) null
          (:`then`
            (set `CharacterMovementComponent.MaxWalkSpeed` 250.0 _charactermovement))
          (:`OnFail`
            (set `CharacterMovementComponent.MaxWalkSpeed` 180.0 _charactermovement)
            (`self.Walk`))))
      (:`then_1`
        (`/Engine/EditorBlueprintResources/StandardMacros.DoOnce` false
          (:`Completed`
            (`GameplayStatics.PlaySound2D` "/Game/AI/Gardes/Level2/GardesDebut/Audio/Alarm_lvl_2_.Alarm_lvl_2_" 1.0 1.0 0.0 null null)))))))

(event `RaycastFront`
  (bind _aipos (`self.AIPos`))
  ;[0.6719 0.00802 0] Raycast front to trigger the alert 2
  (if (not (`self.LightClose`))
    (bind _outhit (`KismetSystemLibrary.SphereTraceSingleByProfile` _aipos (+ _aipos (* (`self.GetActorForwardVector`) 300)) 90.0 "Pawn"))
    (if (== (`GameplayStatics.GetObjectClass` (`.HitActor` (`GameplayStatics.BreakHitResult` _outhit))) "/Game/ThirdPerson/Blueprints/BP_ThirdPersonCharacter.BP_ThirdPersonCharacter_C")
      (set `self.Suspition` 5.0)
      (`self.OnAlertLevel2`))))

(event `self.ReceiveBeginPlay`
  (`|ExecutionSequence`
    (:`then_0`
      ;[0 0.2482 1] Set initial position + ref to the anim blueprint
      (set `self.AIInitPosition` (`self.K2_GetActorLocation`))
      (bind _asanim_blueprint_garde_random_level_2 (cast `/Game/AI/Gardes/Animation/Level2/AnimBlueprint_GardeRandomLevel2` (`SkeletalMeshComponent.GetAnimInstance` (`self.Mesh`))))
      (set `self.As Anim Blueprint Garde` _asanim_blueprint_garde_random_level_2)
      (`self.Walk`))
    (:`then_1`
      (bind _outactors (`GameplayStatics.GetAllActorsOfClass` "/Game/Blueprints/Diversion/Level1/BP_Imprimantes_Level_1.BP_Imprimantes_Level_1_C"))
      (set `self.PrinterPos` (`self.K2_GetActorLocation` (`|GetArrayItem` _outactors))))))

(event `self.PawnSensing.OnSeePawn`
  (params (Pawn :type "Pawn Object Reference"))
  ;[1 0.891 0] Pawn Sensing
  (`self.IncreaseSuspition`))

(event `self.TriggerColliderBack.OnComponentBeginOverlap`
  (params (OverlappedComponent :type "PrimitiveComponent Object Reference") (OtherActor :type "Actor Object Reference") (OtherComp :type "PrimitiveComponent Object Reference") (OtherBodyIndex :type Integer) (bFromSweep :type Boolean) (SweepResult :type "HitResult Structure (by ref)"))
  ;[1 0.3756 0] Trigger guard back
  (bind _asbp_third_person_character (cast `/Game/ThirdPerson/Blueprints/BP_ThirdPersonCharacter` OtherActor))
  (if (not (`/Game/ThirdPerson/Blueprints/BP_ThirdPersonCharacter.isCrouch?` _asbp_third_person_character))
    (`KismetSystemLibrary.Delay` 2.0)
    (`self.OnAlertLevel1`)))

(event `Walk`
  (bind _as_anim_blueprint_garde (`self.As Anim Blueprint Garde`))
  (bind _aipos (`self.AIPos`))
  (bind _returnvalue (`KismetMathLibrary.RandomFloatInRange` (`self.RandomDelayMin`) (`self.RandomDelayMax`)))
  ;[0.02952 1 0] Walk Semi Random
  (`|AIMoveTo` self (`NavigationSystemV1.K2_GetRandomReachablePointInRadius` (`self.AIInitPosition`) (`KismetMathLibrary.RandomFloatInRange` (`self.RandomRadiusMin`) (`self.RandomRadiusMax`)) null null) null
    (:`OnSuccess`
      (bind _outhit (`KismetSystemLibrary.SphereTraceSingleByProfile` :`Start` _aipos :`End` (+ _aipos (* (`self.GetActorForwardVector`) 300)) :`Radius` 90.0 :`ProfileName` "Pawn" :`DrawDebugType` "Persistent"))
      (if (`GameplayStatics.BreakHitResult` _outhit)
        (if (`KismetMathLibrary.RandomBool`)
          (set `/Game/AI/Gardes/Animation/Level2/AnimBlueprint_GardeRandomLevel2.Is Looking` true _as_anim_blueprint_garde)
          (`KismetSystemLibrary.Delay` _returnvalue)
          (set `/Game/AI/Gardes/Animation/Level2/AnimBlueprint_GardeRandomLevel2.Is Looking` false _as_anim_blueprint_garde)
          (else
            (set `/Game/AI/Gardes/Animation/Level2/AnimBlueprint_GardeRandomLevel2.Looking3` true _as_anim_blueprint_garde)
            (`KismetSystemLibrary.Delay` _returnvalue)
            (set `/Game/AI/Gardes/Animation/Level2/AnimBlueprint_GardeRandomLevel2.Looking3` false _as_anim_blueprint_garde)))
        (else
          (set `/Game/AI/Gardes/Animation/Level2/AnimBlueprint_GardeRandomLevel2.Looking2` true _as_anim_blueprint_garde)
          (`KismetSystemLibrary.Delay` _returnvalue)
          (set `/Game/AI/Gardes/Animation/Level2/AnimBlueprint_GardeRandomLevel2.Looking2` false _as_anim_blueprint_garde)))
      (`self.Walk`))
    (:`OnFail`
      (`|AIMoveTo` self (`self.AIInitPosition`) null
        (:`OnSuccess`
          (`self.Walk`))
        (:`OnFail`
          (`self.Walk`))))))

(event `self.TriggerColliderOnGuard.OnComponentBeginOverlap`
  (params (OverlappedComponent :type "PrimitiveComponent Object Reference") (OtherActor :type "Actor Object Reference") (OtherComp :type "PrimitiveComponent Object Reference") (OtherBodyIndex :type Integer) (bFromSweep :type Boolean) (SweepResult :type "HitResult Structure (by ref)"))
  (bind _as_anim_blueprint_garde (`self.As Anim Blueprint Garde`))
  ;[1 0.3943 0] Trigger guard
  (if (not (`/Game/AI/Gardes/Animation/Level2/AnimBlueprint_GardeRandomLevel2.IsElectrocuted` (`self.As Anim Blueprint Garde`)))
    (bind _asbp_third_person_character (cast `/Game/ThirdPerson/Blueprints/BP_ThirdPersonCharacter` OtherActor))
    (cast `/Game/ThirdPerson/Blueprints/BP_ThirdPersonGameMode` (`GameplayStatics.GetGameMode`))
    (set `/Game/AI/Gardes/Animation/Level2/AnimBlueprint_GardeRandomLevel2.Is attack` true _as_anim_blueprint_garde)
    (`self.MoveToInitPos`)
    (`GameplayStatics.PlaySound2D` "/Game/Sound/SFX/Guard/game_over_taser_.game_over_taser_" 1.0 1.0 0.0 null null)
    (`KismetSystemLibrary.Delay` 1.0)
    (`CharacterMovementComponent.DisableMovement` (`self.CharacterMovement`))
    (set `/Game/AI/Gardes/Animation/Level2/AnimBlueprint_GardeRandomLevel2.Is attack` false _as_anim_blueprint_garde)
    (`KismetSystemLibrary.Delay` 8.0)
    (bind _returnvalue (`GameplayStatics.GetCurrentLevelName` true))
    (`GameplayStatics.OpenLevel` (`KismetStringLibrary.Conv_StringToName` _returnvalue))
    (set `/Game/AI/Gardes/Animation/Level2/AnimBlueprint_GardeRandomLevel2.Is attack` false _as_anim_blueprint_garde)
    (set `/Game/ThirdPerson/Blueprints/BP_ThirdPersonCharacter.IsAttacked` false _asbp_third_person_character)))

(event `Extinguisher`
  (if (`self.Exctinguisher`)
    (bind _outactors (`GameplayStatics.GetAllActorsOfClass` "/Game/Blueprints/Diversion/Diversion_Physics/Extinguisher/BP_Extincteur.BP_Extincteur_C"))
    (for _array_element _outactors
      (`|AIMoveTo` self (0.0 0.0 0.0) _array_element 1.0
        (:`OnSuccess`
          (set `self.ExtinguisherIsTrigger` false)
          (`KismetSystemLibrary.Delay` 1.0)
          (`self.Walk`))))))

(event `Distributeur`
  (if (`self.Distributer`)
    (bind _outactors (`GameplayStatics.GetAllActorsOfClass` "/Game/Blueprints/Diversion/Diversion_Physics/BP_distributer.BP_distributer_C"))
    (for _array_element _outactors
      (`|AIMoveTo` self (0.0 0.0 0.0) _array_element 10.0
        (:`OnSuccess`
          (set `self.DistributerIsTrigger` false)
          (`KismetSystemLibrary.Delay` 1.0)
          (`self.Walk`))))))

(event `PrinterEvent`
  (if (`self.Printer`)
    (bind _outactors (`GameplayStatics.GetAllActorsOfClass` "/Game/Blueprints/Diversion/Level1/BP_Imprimantes_Level_1.BP_Imprimantes_Level_1_C"))
    (for _array_element _outactors
      (`|AIMoveTo` self (0.0 0.0 0.0) _array_element 1.0
        (:`OnSuccess`
          (set `self.PrinterIsTrigger` false)
          (`KismetSystemLibrary.Delay` 10.0)
          (`self.Walk`))))))

(event `PhotocopieurEvent`
  (if (`self.Photocopieur`)
    (bind _outactors (`GameplayStatics.GetAllActorsOfClass` "/Game/Blueprints/Diversion/Imprimantes/BP_Photocopier.BP_Photocopier_C"))
    (for _array_element _outactors
      (`|AIMoveTo` self (0.0 0.0 0.0) _array_element
        (:`OnSuccess`
          (set `self.PhotocopieurIsTrigger` false)
          (`KismetSystemLibrary.Delay` 10.0)
          (`self.Walk`))))))

(event `FuseboxEvent`
  (params (ClosestActor :type "Actor Object Reference"))
  (bind _outactors (`GameplayStatics.GetAllActorsOfClass` "/Game/Blueprints/Diversion/Diversion_Physics/FuseBox/BP_FuseBox.BP_FuseBox_C"))
  (for _array_element _outactors
    _)
  (bind _movementresult (`|AIMoveTo` self (0.0 0.0 0.0) _array_element 20.0)
    (:`then`
      (`KismetSystemLibrary.PrintString` (`|GetEnumeratorNameAsString` _movementresult)))
    (:`OnSuccess`
      (`CharacterMovementComponent.DisableMovement` (`self.CharacterMovement`))
      (`KismetSystemLibrary.Delay` 1.0)
      (bind _outactors_2 (`GameplayStatics.GetAllActorsOfClass` "/Game/Blueprints/Diversion/Diversion_Physics/FuseBox/BP_FuseBox.BP_FuseBox_C"))
      (set `/Game/Blueprints/Diversion/Diversion_Physics/FuseBox/BP_FuseBox.Explose` true (`|GetArrayItem` _outactors_2))
      (set `self.FuseBoxIsTrigger` false)
      (set `/Game/AI/Gardes/Animation/Level2/AnimBlueprint_GardeRandomLevel2.IsElectrocuted` true (`self.As Anim Blueprint Garde`))
      (`PawnSensingComponent.SetSensingUpdatesEnabled` (`self.PawnSensing`) false)
      (`ActorComponent.K2_DestroyComponent` (`self.SuspitionATH`)))
    (:`OnFail`
      (`KismetSystemLibrary.PrintString` "Fail"))))

(event `self.ReceiveTick`
  (params (DeltaSeconds :type "Float (single-precision)"))
  (bind (_returnvalue_roll _returnvalue_pitch _returnvalue_yaw) (`KismetMathLibrary.BreakRotator` (`KismetMathLibrary.FindLookAtRotation` (`PlayerCameraManager.GetCameraLocation` (`GameplayStatics.GetPlayerCameraManager` 0)) (`SceneComponent.K2_GetComponentLocation` (`self.SuspitionATH`)))))
  (`/Engine/EditorBlueprintResources/StandardMacros.IsValid` "/Game/AI/Gardes/Level2/GardesRandom/WD_Suspition.WD_Suspition"
    (:`Is Valid`
      (`SceneComponent.K2_SetWorldRotation` (`self.SuspitionATH`) (`KismetMathLibrary.MakeRotator` 0.0 0.0 (+ _returnvalue_yaw 180.0)) false false)
      ;[0 0.04742 1] Event tick
      (`|ExecutionSequence`
        (:`then_0`
          (set `self.AIPos` (`self.K2_GetActorLocation`))
          (if (`/Game/AI/Gardes/Animation/Level2/AnimBlueprint_GardeRandomLevel2.Is attack` (`self.As Anim Blueprint Garde`))
            (`MovementComponent.StopMovementImmediately` (`self.CharacterMovement`)))
          (`self.RaycastFront`)
          (`self.VerifSuspition`))
        (:`then_1`
          (if (`self.ExtinguisherIsTrigger`)
            (`self.Extinguisher`)))
        (:`then_2`
          (if (`self.DistributerIsTrigger`)
            (`self.Distributeur`)))
        (:`then_3`
          (if (`self.PrinterIsTrigger`)
            (`self.PrinterEvent`)))
        (:`then_4`
          (if (`self.PhotocopieurIsTrigger`)
            (`self.PhotocopieurEvent`)))
        (:`then_5`
          (`KismetSystemLibrary.PrintString` (`KismetStringLibrary.Conv_DoubleToString` (`KismetMathLibrary.VSize` (`MovementComponent.Velocity` (`self.CharacterMovement`)))) true true (struct :`G` 0.66 :`B` 1.0 :`A` 1.0) 0.01))))))

(fn `Apprehend`
  (bind _asbp_third_person_character (cast `/Game/ThirdPerson/Blueprints/BP_ThirdPersonCharacter` (`GameplayStatics.GetPlayerCharacter` 0)))
  (`self.K2_DestroyActor` _asbp_third_person_character))

(fn `UserConstructionScript`)