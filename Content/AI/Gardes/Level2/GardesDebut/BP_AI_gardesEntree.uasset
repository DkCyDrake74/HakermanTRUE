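; Stealth guard for the Level 2 entrance that loops through four waypoints with random look-around pauses, chaining AIMoveTo calls without a behavior tree.
; PawnSensing builds suspicion, polled on Tick to trigger investigation, then armed alarm chase.
; A forward sphere trace triggers the chase directly, while a rear trigger prompts investigation of non-crouched players.
; A photocopier flag diverts the guard; center-trigger contact plays an attack and opens level "2".
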(event `self.PawnSensing.OnSeePawn`
  (params (Pawn :type "Pawn Object Reference"))
  (`self.IncreaseSuspition`))

(event `VerifSuspition`
  (`|ExecutionSequence`
    (:`then_0`
      (if (>= (`self.Suspition`) 2.5)
        (`self.OnAlertLevel1`)))
    (:`then_1`
      (if (>= (`self.Suspition`) 5.0)
        (`self.OnAlertLevel2`)))))

(event `IncreaseSuspition`
  (if (<= (`self.Suspition`) (`self.SuspitionMax`))
    (set `self.Suspition` (+ (`self.Suspition`) 0.1))))

(event `OnAlertLevel1`
  (`/Engine/EditorBlueprintResources/StandardMacros.DoOnce` false
    (:`Completed`
      (bind _asbp_third_person_character (cast `/Game/ThirdPerson/Blueprints/BP_ThirdPersonCharacter` (`GameplayStatics.GetPlayerCharacter` 0)))
      (bind _output_get (set `self.PlayerPosition?` (`self.K2_GetActorLocation` _asbp_third_person_character)))
      (`|AIMoveTo` self _output_get null 50.0
        (:`OnSuccess`
          (`KismetSystemLibrary.Delay` (`KismetMathLibrary.RandomFloatInRange` 5.0 10.0))
          (`self.Walk`))))))

(event `SpawnWeapon`
  (`/Engine/EditorBlueprintResources/StandardMacros.DoOnce` false
    (:`Completed`
      (bind _returnvalue (`|SpawnActorFromClass` "/Game/AI/Weapon/BP_Weapon.BP_Weapon_C" (`SceneComponent.GetSocketTransform` (`self.Mesh`) "WeaponSocket" "RTS_World") "Undefined" "OverrideRootScale" null null))
      (`self.K2_AttachToComponent` _returnvalue (`self.Mesh`) "WeaponSocket" "SnapToTarget" "SnapToTarget" "SnapToTarget" true))))

(event `OnAlertLevel2`
  (bind _charactermovement (`self.CharacterMovement`))
  (`self.SpawnWeapon`)
  (`AudioComponent.Play` (`self.Alarm`) 0.0)
  (bind _asbp_third_person_character (cast `/Game/ThirdPerson/Blueprints/BP_ThirdPersonCharacter` (`GameplayStatics.GetPlayerCharacter` 0)))
  (`|AIMoveTo` self (`self.K2_GetActorLocation` _asbp_third_person_character) null
    (:`then`
      (set `CharacterMovementComponent.MaxWalkSpeed` 250.0 _charactermovement))
    (:`OnFail`
      (set `CharacterMovementComponent.MaxWalkSpeed` 180.0 _charactermovement)
      (`self.Walk`))))

(event `RaycastFront`
  (bind _aipos (`self.AIPos`))
  (bind _outhit (`KismetSystemLibrary.SphereTraceSingleByProfile` _aipos (+ _aipos (* (`self.GetActorForwardVector`) 400)) 90.0 "Pawn"))
  (if (== (`GameplayStatics.GetObjectClass` (`.HitActor` (`GameplayStatics.BreakHitResult` _outhit))) "/Game/ThirdPerson/Blueprints/BP_ThirdPersonCharacter.BP_ThirdPersonCharacter_C")
    (`AudioComponent.Play` (`self.Alarm`) 0.0)
    (`self.OnAlertLevel2`)))

(event `PhotocopieurIsTrigger`
  ;[0.1382 0.1412 0.1458] Diversion
  ;;[0.9149 1 0] Photocopieur Diversion
  (bind _returnvalue (`GameplayStatics.GetActorOfClass` "/Game/Blueprints/Diversion/Imprimantes/BP_Photocopier.BP_Photocopier_C"))
  (`|AIMoveTo` self (`/Game/Blueprints/Diversion/Imprimantes/BP_Photocopier.Position` _returnvalue) null
    (:`OnSuccess`
      (`KismetSystemLibrary.Delay` (`/Game/Blueprints/Diversion/Imprimantes/BP_Photocopier.TriggerTime` _returnvalue))
      (set `self.PhotocopieurIsTrigger?` false)
      (`self.Walk`))))

(event `self.TriggerColliderBack.OnComponentBeginOverlap`
  (params (OverlappedComponent :type "PrimitiveComponent Object Reference") (OtherActor :type "Actor Object Reference") (OtherComp :type "PrimitiveComponent Object Reference") (OtherBodyIndex :type Integer) (bFromSweep :type Boolean) (SweepResult :type "HitResult Structure (by ref)"))
  (bind _asbp_third_person_character (cast `/Game/ThirdPerson/Blueprints/BP_ThirdPersonCharacter` OtherActor))
  (if (not (`/Game/ThirdPerson/Blueprints/BP_ThirdPersonCharacter.isCrouch?` _asbp_third_person_character))
    (`AudioComponent.Play` (`self.Spotted`) 0.0)
    (`KismetSystemLibrary.Delay` 2.0)
    (`self.OnAlertLevel1`)))

(event `self.TriggerColliderCenterGuard.OnComponentBeginOverlap`
  (params (OverlappedComponent :type "PrimitiveComponent Object Reference") (OtherActor :type "Actor Object Reference") (OtherComp :type "PrimitiveComponent Object Reference") (OtherBodyIndex :type Integer) (bFromSweep :type Boolean) (SweepResult :type "HitResult Structure (by ref)"))
  (bind _as_anim_blueprint_garde_entree_level_2 (`self.As Anim Blueprint Garde Entree Level 2`))
  (bind _asbp_third_person_character (cast `/Game/ThirdPerson/Blueprints/BP_ThirdPersonCharacter` OtherActor))
  (cast `/Game/ThirdPerson/Blueprints/BP_ThirdPersonGameMode` (`GameplayStatics.GetGameMode`))
  (set `/Game/AI/Gardes/Animation/Level2/AnimBlueprint_GardeEntreeLevel2.Is attack` true _as_anim_blueprint_garde_entree_level_2)
  (`KismetSystemLibrary.Delay` 8.0)
  (`GameplayStatics.OpenLevel` "2")
  (set `/Game/AI/Gardes/Animation/Level2/AnimBlueprint_GardeEntreeLevel2.Is attack` false _as_anim_blueprint_garde_entree_level_2)
  (set `/Game/ThirdPerson/Blueprints/BP_ThirdPersonCharacter.IsAttacked` false _asbp_third_person_character))

(event `self.ReceiveBeginPlay`
  ;[0 1 0.8781] Init walk
  (bind _asanim_blueprint_garde_entree_level_2 (cast `/Game/AI/Gardes/Animation/Level2/AnimBlueprint_GardeEntreeLevel2` (`SkeletalMeshComponent.GetAnimInstance` (`self.Mesh`))))
  (set `self.As Anim Blueprint Garde Entree Level 2` _asanim_blueprint_garde_entree_level_2)
  (`KismetSystemLibrary.Delay` 1.0)
  (`self.Walk`))

(event `Walk`
  (bind _as_anim_blueprint_garde_entree_level_2 (`self.As Anim Blueprint Garde Entree Level 2`))
  ;[0.001953 0 1] Walk Waypoints
  (bind _returnvalue (`GameplayStatics.GetActorOfClass` "/Game/AI/Gardes/Level2/GardesDebut/Waypoints/WaypointsDebut.WaypointsDebut_C"))
  (`|AIMoveTo` self (0.0 0.0 0.0) _returnvalue
    (:`OnSuccess`
      (set `/Game/AI/Gardes/Animation/Level2/AnimBlueprint_GardeEntreeLevel2.Is Looking` true _as_anim_blueprint_garde_entree_level_2)
      (`KismetSystemLibrary.Delay` (`KismetMathLibrary.RandomFloatInRange` 3.0 7.0))
      (set `/Game/AI/Gardes/Animation/Level2/AnimBlueprint_GardeEntreeLevel2.Is Looking` false _as_anim_blueprint_garde_entree_level_2)
      (bind _returnvalue_2 (`GameplayStatics.GetActorOfClass` "/Game/AI/Gardes/Level2/GardesDebut/Waypoints/WaypointsDebut1.WaypointsDebut1_C"))
      (`|AIMoveTo` self (0.0 0.0 0.0) _returnvalue_2
        (:`OnSuccess`
          (set `/Game/AI/Gardes/Animation/Level2/AnimBlueprint_GardeEntreeLevel2.Is Looking` true _as_anim_blueprint_garde_entree_level_2)
          (`KismetSystemLibrary.Delay` (`KismetMathLibrary.RandomFloatInRange` 3.0 7.0))
          (set `/Game/AI/Gardes/Animation/Level2/AnimBlueprint_GardeEntreeLevel2.Is Looking` false _as_anim_blueprint_garde_entree_level_2)
          (bind _returnvalue_3 (`GameplayStatics.GetActorOfClass` "/Game/AI/Gardes/Level2/GardesDebut/Waypoints/WaypointsDebut2.WaypointsDebut2_C"))
          (`|AIMoveTo` self (0.0 0.0 0.0) _returnvalue_3
            (:`OnSuccess`
              (set `/Game/AI/Gardes/Animation/Level2/AnimBlueprint_GardeEntreeLevel2.Is Looking` true _as_anim_blueprint_garde_entree_level_2)
              (`KismetSystemLibrary.Delay` (`KismetMathLibrary.RandomFloatInRange` 3.0 7.0))
              (set `/Game/AI/Gardes/Animation/Level2/AnimBlueprint_GardeEntreeLevel2.Is Looking` false _as_anim_blueprint_garde_entree_level_2)
              (bind _returnvalue_4 (`GameplayStatics.GetActorOfClass` "/Game/AI/Gardes/Level2/GardesDebut/Waypoints/WaypointsDebut3.WaypointsDebut3_C"))
              (`|AIMoveTo` self (0.0 0.0 0.0) _returnvalue_4
                (:`OnSuccess`
                  (set `/Game/AI/Gardes/Animation/Level2/AnimBlueprint_GardeEntreeLevel2.Is Looking` true _as_anim_blueprint_garde_entree_level_2)
                  (`KismetSystemLibrary.Delay` (`KismetMathLibrary.RandomFloatInRange` 3.0 7.0))
                  (set `/Game/AI/Gardes/Animation/Level2/AnimBlueprint_GardeEntreeLevel2.Is Looking` false _as_anim_blueprint_garde_entree_level_2)
                  (`self.Walk`))))))))))

(event `self.ReceiveTick`
  (params (DeltaSeconds :type "Float (single-precision)"))
  ;[1 0 0.8206] Verif Diversion
  (set `self.AIPos` (`self.K2_GetActorLocation`))
  (`|ExecutionSequence`
    (:`then_0`
      (if (`self.PhotocopieurIsTrigger?`)
        (`self.PhotocopieurIsTrigger`)))
    (:`then_1`
      (`self.RaycastFront`)
      (`self.VerifSuspition`))))

(fn `Apprehend`
  (bind _asbp_third_person_character (cast `/Game/ThirdPerson/Blueprints/BP_ThirdPersonCharacter` (`GameplayStatics.GetPlayerCharacter` 0)))
  (`self.K2_DestroyActor` _asbp_third_person_character))

(fn `UserConstructionScript`)