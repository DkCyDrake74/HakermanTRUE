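; Player-triggered scan ability that outlines level devices (webcams, printers, routers, distributors) and the player for a limited time, followed by a cooldown.
; Scan enables the "Scan"-tagged post-process volume, feeds player position and a Timeline-driven radius into PC_Outline, and toggles Custom Depth on target meshes.
; Self-retriggering timer events count down duration and cooldown with debug prints.
; The security camera highlight in ScanDiversion is disconnected.
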(event `InputAction|Scan`
  (params (Key :type "Key Structure"))
  (:`Pressed`
    (`self.Scan`)))

(event `Scan`
  (if (`self.CanScan?`)
    (set `self.CanScan?` false)
    (bind _outactors (`GameplayStatics.GetAllActorsOfClassWithTag` "/Script/Engine.PostProcessVolume" "Scan"))
    (set `PostProcessVolume.bEnabled` true (`|GetArrayItem` _outactors))
    (bind _asbp_third_person_character (cast `/Game/ThirdPerson/Blueprints/BP_ThirdPersonCharacter` (`GameplayStatics.GetPlayerCharacter` 0)))
    (bind _mesh (`Character.Mesh` _asbp_third_person_character))
    (`KismetMaterialLibrary.SetVectorParameterValue` "/Game/Blueprints/Scan2/PC_Outline.PC_Outline" "Position" (`KismetMathLibrary.Conv_VectorToLinearColor` (`SceneComponent.K2_GetComponentLocation` _mesh)))
    (`self.StartTimerScan`)
    (bind _outactors_2 (`GameplayStatics.GetAllActorsOfClass` "/Game/PostProcess/BP_ScanLevel1.BP_ScanLevel1_C"))
    (`self.ScanDiversion` true)
    (`PrimitiveComponent.SetRenderCustomDepth` _mesh true)
    (bind (_direction _newtrack_0) (`Timeline|Timeline` :!via `Reverse` :!label _label)
      (:`Update`
        (`KismetMaterialLibrary.SetScalarParameterValue` "/Game/Blueprints/Scan2/PC_Outline.PC_Outline" "Radius" _newtrack_0)))))

(event `StartTimerScan`
  (bind _returnvalue (`KismetSystemLibrary.K2_SetTimerDelegate` (delegate `StartTimerScan`) 0.1 true))
  (set `self.ScanTimerHandle` _returnvalue)
  (if (<= (`self.CurrentTimeScan`) 0.0)
    (`self.StopScanTimer`)
    (set `self.CurrentTimeScan` 5.0)
    (`self.StartScanCooldown`)
    (bind _outactors (`GameplayStatics.GetAllActorsOfClass` "/Game/PostProcess/BP_ScanLevel1.BP_ScanLevel1_C"))
    (`self.ScanDiversion` false)
    (`PrimitiveComponent.SetRenderCustomDepth` (`Character.Mesh` (stale `Scan` _asbp_third_person_character)) false)
    (goto _label)
    (else
      (bind _output_get (set `self.CurrentTimeScan` (- (`self.CurrentTimeScan`) 0.1)))
      (`KismetSystemLibrary.PrintString` (`KismetStringLibrary.Concat_StrStr` "Scan time remain : " (`KismetStringLibrary.Conv_DoubleToString` _output_get)) true true (struct :`G` 0.66 :`B` 1.0 :`A` 1.0) 0.1))))

(event `StopScanTimer`
  (`KismetSystemLibrary.K2_ClearAndInvalidateTimerHandle` (`self.ScanTimerHandle`)))

(event `StartScanCooldown`
  (bind _returnvalue (`KismetSystemLibrary.K2_SetTimerDelegate` (delegate `StartScanCooldown`) 0.1 true))
  (set `self.ScanCooldownHandle` _returnvalue)
  (if (>= (`self.CurrentCooldownScan`) 5.0)
    (`KismetSystemLibrary.K2_ClearAndInvalidateTimerHandle` (`self.ScanCooldownHandle`))
    (set `self.CanScan?` true)
    (set `self.CurrentCooldownScan` 0.0)
    (else
      (bind _output_get (set `self.CurrentCooldownScan` (+ (`self.CurrentCooldownScan`) 0.1)))
      (`KismetSystemLibrary.PrintString` (`KismetStringLibrary.Concat_StrStr` "Scan cooldown : " (`KismetStringLibrary.Conv_DoubleToString` _output_get)) true true (struct :`G` 0.66 :`B` 1.0 :`A` 1.0) 0.1))))

(fn `ScanDiversion`
  (params (Scan :type Boolean))
  (`|ExecutionSequence`
    (:`then_0`
      (bind _outactors (`GameplayStatics.GetAllActorsOfClass` "/Game/Blueprints/Camera/Camera/Level0/BP_Webcam_0_1.BP_Webcam_0_1_C"))
      (for _array_element _outactors
        (`PrimitiveComponent.SetRenderCustomDepth` (`/Game/Blueprints/Camera/Camera/Level0/BP_Webcam_0_1.SM_Laptop_01` _array_element) Scan)))
    (:`then_1`
      (bind _outactors_2 (`GameplayStatics.GetAllActorsOfClass` "/Game/Blueprints/Camera/Camera/Level0/BP_Camera_0_1.BP_Camera_0_1_C"))
      (for _array_element_2 _outactors_2
        _))
    (:`then_2`
      (bind _outactors_3 (`GameplayStatics.GetAllActorsOfClass` "/Game/Blueprints/Diversion/Level1/BP_Imprimantes_Level_1.BP_Imprimantes_Level_1_C"))
      (for _array_element_3 _outactors_3
        (`PrimitiveComponent.SetRenderCustomDepth` (`/Game/Blueprints/Diversion/Level1/BP_Imprimantes_Level_1.SM_Printer` _array_element_3) Scan)))
    (:`then_3`
      (bind _outactors_4 (`GameplayStatics.GetAllActorsOfClass` "/Game/Blueprints/Diversion/DiversionReseau/BP_Router.BP_Router_C"))
      (for _array_element_4 _outactors_4
        (`PrimitiveComponent.SetRenderCustomDepth` (`/Game/Blueprints/Diversion/DiversionReseau/BP_Router.SM_ElectricMeterSet01Base` _array_element_4) Scan)
        (`PrimitiveComponent.SetRenderCustomDepth` (`/Game/Blueprints/Diversion/DiversionReseau/BP_Router.SM_ElectricMeterSet01Box` _array_element_4) Scan)))
    (:`then_4`
      (bind _outactors_5 (`GameplayStatics.GetAllActorsOfClass` "/Game/Blueprints/Diversion/Diversion_Physics/BP_distributer.BP_distributer_C"))
      (for _array_element_5 _outactors_5
        (`PrimitiveComponent.SetRenderCustomDepth` (`/Game/Blueprints/Diversion/Diversion_Physics/BP_distributer.Cube` _array_element_5) Scan)))))

(fn `ScanFirstSide`
  (set `self.Computer` true)
  (set `self.Photocopieur` false))

(fn `ScanSecondSide`
  (set `self.Computer` false)
  (set `self.Photocopieur` true))

(fn `UserConstructionScript`)