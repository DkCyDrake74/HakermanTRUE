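; BP_DIversionScan is a Blueprint in the PostProcess folder that switches Custom Depth rendering on or off for diversion objects, presumably for a scan highlight.
; Its ScanDiversion function takes a boolean and applies it to the laptop, printer and cube meshes of the webcam, printer and distributor Blueprints.
; Each target is found with Get All Actors Of Class, and only the first instance of each class is affected, with no validity check.
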(fn `ScanDiversion`
  (params (RenderCustomDepth :type Boolean))
  (`|ExecutionSequence`
    (:`then_0`
      (bind _outactors (`GameplayStatics.GetAllActorsOfClass` "/Game/Blueprints/Camera/Camera/Level0/BP_Webcam_0_1.BP_Webcam_0_1_C"))
      (`PrimitiveComponent.SetRenderCustomDepth` (`/Game/Blueprints/Camera/Camera/Level0/BP_Webcam_0_1.SM_Laptop_01` (`|GetArrayItem` _outactors)) RenderCustomDepth))
    (:`then_1`
      (bind _outactors_2 (`GameplayStatics.GetAllActorsOfClass` "/Game/Blueprints/Diversion/Level1/BP_Imprimantes_Level_1.BP_Imprimantes_Level_1_C"))
      (`PrimitiveComponent.SetRenderCustomDepth` (`/Game/Blueprints/Diversion/Level1/BP_Imprimantes_Level_1.SM_Printer` (`|GetArrayItem` _outactors_2)) RenderCustomDepth))
    (:`then_2`
      (bind _outactors_3 (`GameplayStatics.GetAllActorsOfClass` "/Game/Blueprints/Diversion/Diversion_Physics/BP_distributer.BP_distributer_C"))
      (`PrimitiveComponent.SetRenderCustomDepth` (`/Game/Blueprints/Diversion/Diversion_Physics/BP_distributer.Cube` (`|GetArrayItem` _outactors_3)) RenderCustomDepth))))

(fn `UserConstructionScript`)