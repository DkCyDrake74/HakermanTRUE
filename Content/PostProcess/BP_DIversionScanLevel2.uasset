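; Diversion scan actor for level 2 that toggles custom depth on interactive props, presumably for a post-process highlight.
; ScanDiversion applies the Scan flag to webcam laptops, printer, cameras, computer monitors, photocopiers and doors found by class.
; Booleans gate each webcam, the printer and photocopiers (via Computer); cameras, monitors and doors always follow Scan.
; Webcams and printer are picked by fixed array index, so they depend on actor lookup order.
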(fn `ScanDiversion`
  (params (Scan :type Boolean))
  (`|ExecutionSequence`
    (:`then_0`
      (bind _outactors (`GameplayStatics.GetAllActorsOfClass` "/Game/Blueprints/Camera/Camera/Level1/Webcam_Level_1/BP_Webcam_1_1.BP_Webcam_1_1_C"))
      (`|ExecutionSequence`
        (:`then_0`
          (if (`self.Webcam_2`)
            (`PrimitiveComponent.SetRenderCustomDepth` (`/Game/Blueprints/Camera/Camera/Level1/Webcam_Level_1/BP_Webcam_1_1.SM_Laptop_01` (`|GetArrayItem` _outactors)) Scan)))
        (:`then_1`
          (if (`self.Webcam_1`)
            (`PrimitiveComponent.SetRenderCustomDepth` (`/Game/Blueprints/Camera/Camera/Level1/Webcam_Level_1/BP_Webcam_1_1.SM_Laptop_01` (`|GetArrayItem` _outactors 1)) Scan)))
        (:`then_2`
          (if (`self.Webcam_3`)
            (`PrimitiveComponent.SetRenderCustomDepth` (`/Game/Blueprints/Camera/Camera/Level1/Webcam_Level_1/BP_Webcam_1_1.SM_Laptop_01` (`|GetArrayItem` _outactors 2)) Scan)))))
    (:`then_1`
      (bind _outactors_2 (`GameplayStatics.GetAllActorsOfClass` "/Game/Blueprints/Diversion/Level1/BP_Imprimantes_Level_1.BP_Imprimantes_Level_1_C"))
      (if (`self.Printer`)
        (`PrimitiveComponent.SetRenderCustomDepth` (`/Game/Blueprints/Diversion/Level1/BP_Imprimantes_Level_1.SM_Printer` (`|GetArrayItem` _outactors_2)) Scan)))
    (:`then_2`
      (bind _outactors_3 (`GameplayStatics.GetAllActorsOfClass` "/Game/Blueprints/Camera/Camera/Level1/Camera_Level_1/BP_Camera_1_1.BP_Camera_1_1_C"))
      (for _array_element _outactors_3
        (`PrimitiveComponent.SetRenderCustomDepth` (`/Game/Blueprints/Camera/Camera/Level1/Camera_Level_1/BP_Camera_1_1.SM_SecurityCameraSet02` _array_element) Scan)))
    (:`then_3`
      (bind _outactors_4 (`GameplayStatics.GetAllActorsOfClass` "/Game/Blueprints/Ordinateur_mails/Level1/BP_Ordinateurs.BP_Ordinateurs_C"))
      (for _array_element_2 _outactors_4
        (`PrimitiveComponent.SetRenderCustomDepth` (`/Game/Blueprints/Ordinateur_mails/Level1/BP_Ordinateurs.SM_Monitor_01` _array_element_2) Scan)))
    (:`then_4`
      (bind _outactors_5 (`GameplayStatics.GetAllActorsOfClass` "/Game/Blueprints/Diversion/Imprimantes/BP_Photocopier.BP_Photocopier_C"))
      (for _array_element_3 _outactors_5
        (if (`self.Computer`)
          (`PrimitiveComponent.SetRenderCustomDepth` (`/Game/Blueprints/Diversion/Imprimantes/BP_Photocopier.SM_Photocopier_01` _array_element_3) Scan))))
    (:`then_5`
      (bind _outactors_6 (`GameplayStatics.GetAllActorsOfClass` "/Game/Blueprints/Digicode_door/Level1/BP_Door_1_1.BP_Door_1_1_C"))
      (for _array_element_4 _outactors_6
        (`PrimitiveComponent.SetRenderCustomDepth` (`/Game/Blueprints/Digicode_door/Level1/BP_Door_1_1.Porte` _array_element_4) Scan)))))

(fn `UserConstructionScript`)