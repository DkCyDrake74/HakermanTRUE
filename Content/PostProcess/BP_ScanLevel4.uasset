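; BP_ScanLevel4 is a timed scan ability that highlights webcams, cameras, photocopiers, doors, guards and the player through custom depth.
; The Scan input enables the tagged post-process volume and drives PC_Outline's position and radius, using a Timeline for the radius.
; Looping timers run the scan duration and cooldown, printing both.
; ScanFirstSide and ScanSecondSide toggle photocopier highlighting; the computer branch is empty.
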(event `InputAction|Scan`
  (params (Key :type "Key Structure"))
  (:`Pressed`
    (if (`self.CanScan?`)
      (set `self.CanScan?` false)
      (bind _outactors (`GameplayStatics.GetAllActorsOfClassWithTag` "/Script/Engine.PostProcessVolume" "Scan"))
      (set `PostProcessVolume.bEnabled` true (`|GetArrayItem` _outactors))
      (bind _asbp_third_person_character (cast `/Game/ThirdPerson/Blueprints/BP_ThirdPersonCharacter` (`GameplayStatics.GetPlayerCharacter` 0)))
      (bind _mesh (`Character.Mesh` _asbp_third_person_character))
      (`KismetMaterialLibrary.SetVectorParameterValue` "/Game/Blueprints/Scan2/PC_Outline.PC_Outline" "Position" (`KismetMathLibrary.Conv_VectorToLinearColor` (`SceneComponent.K2_GetComponentLocation` _mesh)))
      (`self.StartTimerScan`)
      (bind _outactors_2 (`GameplayStatics.GetAllActorsOfClass` "BP_ScanLevel4_C"))
      (`self.ScanDiversion` (`|GetArrayItem` _outactors_2) true)
      (`PrimitiveComponent.SetRenderCustomDepth` _mesh true)
      (bind (_direction _newtrack_0) (`Timeline|Timeline` :!via `Reverse` :!label _label)
        (:`Update`
          (`KismetMaterialLibrary.SetScalarParameterValue` "/Game/Blueprints/Scan2/PC_Outline.PC_Outline" "Radius" _newtrack_0))))))

(event `StartTimerScan`
  (bind _returnvalue (`KismetSystemLibrary.K2_SetTimerDelegate` (delegate `StartTimerScan`) 0.1 true))
  (set `self.ScanTimerHandle` _returnvalue)
  (if (<= (`self.CurrentTimeScan`) 0.0)
    (`self.StopScanTimer`)
    (set `self.CurrentTimeScan` 5.0)
    (`self.StartScanCooldown`)
    (bind _outactors (`GameplayStatics.GetAllActorsOfClass` "BP_ScanLevel4_C"))
    (`self.ScanDiversion` (`|GetArrayItem` _outactors) false)
    (`PrimitiveComponent.SetRenderCustomDepth` (`Character.Mesh` (stale `InputAction|Scan` _asbp_third_person_character)) false)
    (goto _label)
    (else
      (bind _output_get (set `self.CurrentTimeScan` (- (`self.CurrentTimeScan`) 0.1)))
      (`KismetSystemLibrary.PrintString` (`KismetStringLibrary.Concat_StrStr` "Scan time remain : " (`KismetStringLibrary.Conv_DoubleToString` _output_get)) true true (struct :`G` 0.66 :`B` 1.0 :`A` 1.0) 0.1))))

(event `StopScanTimer`
  (`KismetSystemLibrary.K2_ClearAndInvalidateTimerHandle` (`self.ScanTimerHandle`)))

(event `StartScanCooldown`
  (bind _returnvalue (`KismetSystemLibrary.K2_SetTimerDelegate` (delegate `StartScanCooldown`) 0.1 true))
  (set `self.ScanCooldownHandle` _returnvalue)
  (if (>= (`self.CurrentCooldownScan`) 5.0)
    (`KismetSystemLibrary.K2_ClearAndInvalidateTimerHandle` (`self.ScanCooldownHandle`))
    (set `self.CanScan?` true)
    (set `self.CurrentCooldownScan` 0.0)
    (else
      (bind _output_get (set `self.CurrentCooldownScan` (+ (`self.CurrentCooldownScan`) 0.1)))
      (`KismetSystemLibrary.PrintString` (`KismetStringLibrary.Concat_StrStr` "Scan cooldown : " (`KismetStringLibrary.Conv_DoubleToString` _output_get)) true true (struct :`G` 0.66 :`B` 1.0 :`A` 1.0) 0.1))))

(fn `ScanDiversion`
  (params (Scan :type Boolean))
  (`|ExecutionSequence`
    (:`then_0`
      (bind _outactors (`GameplayStatics.GetAllActorsOfClass` "/Game/Blueprints/Camera/Camera/Level1/Webcam_Level_1/BP_Webcam_1_1.BP_Webcam_1_1_C"))
      (for _array_element _outactors
        (`PrimitiveComponent.SetRenderCustomDepth` (`/Game/Blueprints/Camera/Camera/Level1/Webcam_Level_1/BP_Webcam_1_1.SM_Laptop_01` _array_element) Scan)))
    (:`then_1`
      (bind _outactors_2 (`GameplayStatics.GetAllActorsOfClass` "/Game/Blueprints/Ordinateur_mails/Level1/BP_Ordinateurs1.BP_Ordinateurs1_C"))
      (if (`self.Computer`)
        _))
    (:`then_2`
      (bind _outactors_3 (`GameplayStatics.GetAllActorsOfClass` "/Game/Blueprints/Camera/Camera/Level1/Camera_Level_1/BP_Camera_1_1.BP_Camera_1_1_C"))
      (for _array_element_2 _outactors_3
        (`PrimitiveComponent.SetRenderCustomDepth` (`/Game/Blueprints/Camera/Camera/Level1/Camera_Level_1/BP_Camera_1_1.SM_SecurityCameraSet02` _array_element_2) Scan)))
    (:`then_3`
      (bind _outactors_4 (`GameplayStatics.GetAllActorsOfClass` "/Game/Blueprints/Diversion/Imprimantes/BP_Photocopier.BP_Photocopier_C"))
      (for _array_element_3 _outactors_4
        (if (`self.Photocopieur`)
          (`PrimitiveComponent.SetRenderCustomDepth` (`/Game/Blueprints/Diversion/Imprimantes/BP_Photocopier.SM_Photocopier_01` _array_element_3) Scan))))
    (:`then_4`
      (bind _outactors_5 (`GameplayStatics.GetAllActorsOfClass` "/Game/Blueprints/Digicode_door/Level1/BP_Door_1_1.BP_Door_1_1_C"))
      (for _array_element_4 _outactors_5
        (`PrimitiveComponent.SetRenderCustomDepth` (`/Game/Blueprints/Digicode_door/Level1/BP_Door_1_1.Porte` _array_element_4) Scan)))
    (:`then_5`
      (bind _outactors_6 (`GameplayStatics.GetAllActorsOfClass` "/Game/AI/Gardes/Level2/GardesRandom/BP_AI_gardes_Level_2.BP_AI_gardes_Level_2_C"))
      (for _array_element_5 _outactors_6
        (`PrimitiveComponent.SetRenderCustomDepth` (`Character.Mesh` _array_element_5) Scan)))))

(fn `ScanFirstSide`
  (set `self.Computer` true)
  (set `self.Photocopieur` false))

(fn `ScanSecondSide`
  (set `self.Computer` false)
  (set `self.Photocopieur` true))

(fn `UserConstructionScript`)