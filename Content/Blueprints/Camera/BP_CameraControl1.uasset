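; BP_CameraControl1 turns BP_Camera_1_1 actors horizontally with mouse X input while the third-person character's UI is inactive.
; Each MouseX event finds every such camera and clamps the axis value to ±20.
; It makes two relative yaw additions per camera, one gated on yaw below 180 and one on yaw above 0, so both apply when both checks pass.
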(event `InputAxisKey|MouseX` :consume false
  (params (AxisValue :type "Float (single-precision)"))
  (bind _returnvalue (`KismetMathLibrary.FClamp` AxisValue -20.0 20.0))
  (bind _asbp_third_person_character (cast `/Game/ThirdPerson/Blueprints/BP_ThirdPersonCharacter` (`GameplayStatics.GetPlayerCharacter` 0)))
  (if (not (`/Game/ThirdPerson/Blueprints/BP_ThirdPersonCharacter.UiIsActive` _asbp_third_person_character))
    (bind _outactors (`GameplayStatics.GetAllActorsOfClass` "/Game/Blueprints/Camera/Camera/Level1/Camera_Level_1/BP_Camera_1_1.BP_Camera_1_1_C"))
    (for _array_element _outactors
      (bind (_returnvalue_roll _returnvalue_pitch _returnvalue_yaw) (`KismetMathLibrary.BreakRotator` (`self.K2_GetActorRotation` _array_element)))
      (bind _output_get (set `self.rotationValidMax` (< _returnvalue_yaw 180.0)))
      (bind _output_get_2 (set `self.rotationValidMin` (> _returnvalue_yaw 0.0)))
      (bind _rootcomponent (`Actor.RootComponent` _array_element))
      (bind (_returnvalue_roll_2 _returnvalue_pitch_2 _returnvalue_yaw_2) (`KismetMathLibrary.BreakRotator` (`KismetMathLibrary.SelectRotator` (`KismetMathLibrary.MakeRotator` 0.0 0.0 (`KismetMathLibrary.SelectFloat` _returnvalue 0.0 _output_get)) (`KismetMathLibrary.MakeRotator` 0.0) true)))
      (`SceneComponent.K2_AddRelativeRotation` _rootcomponent (`KismetMathLibrary.MakeRotator` 0.0 0.0 _returnvalue_yaw_2) false false)
      (bind (_returnvalue_roll_3 _returnvalue_pitch_3 _returnvalue_yaw_3) (`KismetMathLibrary.BreakRotator` (`KismetMathLibrary.SelectRotator` (`KismetMathLibrary.MakeRotator` 0.0) (`KismetMathLibrary.MakeRotator` 0.0 0.0 (`KismetMathLibrary.SelectFloat` _returnvalue 0.0 _output_get_2)))))
      (`SceneComponent.K2_AddRelativeRotation` _rootcomponent (`KismetMathLibrary.MakeRotator` 0.0 0.0 _returnvalue_yaw_3) false false))))

(fn `UserConstructionScript`)