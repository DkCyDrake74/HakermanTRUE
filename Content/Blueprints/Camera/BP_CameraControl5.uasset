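; BP_CameraControl5 lets horizontal mouse movement pan the player's current camera view target.
; MouseX input above a small threshold is ignored while character UI is active or the tagged StartCamera is viewed.
; Clamped input feeds two relative yaw rotations, each gated by a yaw check against 0 or 180 degrees.
; A DoOnce with a delayed reset throttles the camera movement sound.
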(event `InputAxisKey|MouseX` :consume false
  (params (AxisValue :type "Float (single-precision)"))
  (bind _returnvalue (`KismetMathLibrary.FClamp` AxisValue -20.0 20.0))
  (bind _returnvalue_2 (`Controller.GetViewTarget` (`GameplayStatics.GetPlayerController` 0)))
  (bind (_returnvalue_roll _returnvalue_pitch _returnvalue_yaw) (`KismetMathLibrary.BreakRotator` (`self.K2_GetActorRotation` _returnvalue_2)))
  (bind _rootcomponent (`Actor.RootComponent` _returnvalue_2))
  (bind _asbp_third_person_character (cast `/Game/ThirdPerson/Blueprints/BP_ThirdPersonCharacter` (`GameplayStatics.GetPlayerCharacter` 0)))
  (if (`/Game/ThirdPerson/Blueprints/BP_ThirdPersonCharacter.UiIsActive` _asbp_third_person_character)
    _
    (elif (>= (`KismetMathLibrary.Abs` AxisValue) 0.9)
      (`|ExecutionSequence`
        (:`then_0`
          (bind _outactors (`GameplayStatics.GetAllActorsOfClassWithTag` "/Script/Engine.CameraActor" "StartCamera"))
          (if (not (== _returnvalue_2 (`|GetArrayItem` _outactors)))
            (`|ExecutionSequence`
              (:`then_0`
                (bind _output_get (set `self.rotationValidMax` (< _returnvalue_yaw 180.0)))
                (bind _output_get_2 (set `self.rotationValidMin` (> _returnvalue_yaw 0.0)))
                (bind (_returnvalue_roll_2 _returnvalue_pitch_2 _returnvalue_yaw_2) (`KismetMathLibrary.BreakRotator` (`KismetMathLibrary.SelectRotator` (`KismetMathLibrary.MakeRotator` 0.0 0.0 (`KismetMathLibrary.SelectFloat` _returnvalue 0.0 _output_get)) (`KismetMathLibrary.MakeRotator` 0.0) true)))
                (`SceneComponent.K2_AddRelativeRotation` _rootcomponent (`KismetMathLibrary.MakeRotator` 0.0 0.0 _returnvalue_yaw_2) false false)
                (bind (_returnvalue_roll_3 _returnvalue_pitch_3 _returnvalue_yaw_3) (`KismetMathLibrary.BreakRotator` (`KismetMathLibrary.SelectRotator` (`KismetMathLibrary.MakeRotator` 0.0) (`KismetMathLibrary.MakeRotator` 0.0 0.0 (`KismetMathLibrary.SelectFloat` _returnvalue 0.0 _output_get_2)))))
                (`SceneComponent.K2_AddRelativeRotation` _rootcomponent (`KismetMathLibrary.MakeRotator` 0.0 0.0 _returnvalue_yaw_3) false false))
              (:`then_1`
                (`/Engine/EditorBlueprintResources/StandardMacros.DoOnce` false :!label _label
                  (:`Completed`
                    (`GameplayStatics.PlaySound2D` "/Game/Sound/SFX/Camera/Camera_Move_Cue.Camera_Move_Cue" 1.0 1.0 0.0 null null)
                    (`KismetSystemLibrary.Delay` 1.9)
                    (goto _label :!via `Reset`)))))))))))

(fn `UserConstructionScript`)