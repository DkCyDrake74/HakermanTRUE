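; BP_Camera_Allow2 holds on/off permission flags for the "2" set of eight cameras and five webcams.
; AllowCamera and AllowWebcam each overwrite their whole group of flags from boolean inputs.
; BeginPlay calls AllowCamera with only the first camera enabled; AllowWebcam is not called within this Blueprint.
; It contains no camera switching logic, only the stored state.
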(event `self.ReceiveBeginPlay`
  (`self.AllowCamera` true))

(fn `AllowCamera`
  (params (`Camera 1` :type Boolean) (`Camera 2` :type Boolean) (`Camera 3` :type Boolean) (`Camera 4` :type Boolean) (`Camera 5` :type Boolean) (`Camera 6` :type Boolean) (`Camera 7` :type Boolean) (`Camera 8` :type Boolean))
  (set `self.Allow_Camera2_1` `Camera 1`)
  (set `self.Allow_Camera2_2` `Camera 2`)
  (set `self.Allow_Camera2_3` `Camera 3`)
  (set `self.Allow_Camera2_4` `Camera 4`)
  (set `self.Allow_Camera2_5` `Camera 5`)
  (set `self.Allow_Camera2_6` `Camera 6`)
  (set `self.Allow_Camera2_7` `Camera 7`)
  (set `self.Allow_Camera2_8` `Camera 8`))

(fn `AllowWebcam`
  (params (`Webcam 1` :type Boolean) (`Webcam 2` :type Boolean) (`Webcam 3` :type Boolean) (`Webcam 4` :type Boolean) (`Webcam 5` :type Boolean))
  (set `self.Allow_Webcam2_1` `Webcam 1`)
  (set `self.Allow_Webcam2_2` `Webcam 2`)
  (set `self.Allow_Webcam2_3` `Webcam 3`)
  (set `self.Allow_Webcam2_4` `Webcam 4`)
  (set `self.Allow_Webcam2_5` `Webcam 5`))

(fn `UserConstructionScript`)