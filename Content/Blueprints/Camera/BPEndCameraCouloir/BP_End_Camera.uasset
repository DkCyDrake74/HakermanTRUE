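; BP_End_Camera is a trigger actor that switches the player's view for the end-of-corridor camera.
; Each Box begin overlap alternates through a FlipFlop, with no filter on the overlapping actor.
; The first branch sets the view target to the first EndCamera actor and enables its CanMove flag.
; The second returns the view to the actor tagged Webcam4 and disables CanMove.
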(event `self.Box.OnComponentBeginOverlap`
  (params (OverlappedComponent :type "PrimitiveComponent Object Reference") (OtherActor :type "Actor Object Reference") (OtherComp :type "PrimitiveComponent Object Reference") (OtherBodyIndex :type Integer) (bFromSweep :type Boolean) (SweepResult :type "HitResult Structure (by ref)"))
  (`/Engine/EditorBlueprintResources/StandardMacros.FlipFlop`
    (:`A`
      (bind _outactors (`GameplayStatics.GetAllActorsOfClass` "/Game/Blueprints/Camera/Camera/Level1/EndCamera.EndCamera_C"))
      (`PlayerController.SetViewTargetWithBlend` (`GameplayStatics.GetPlayerController` 0) (`|GetArrayItem` _outactors) 0.0 "VTBlend_Linear" 0.0 false)
      (bind _outactors_2 (`GameplayStatics.GetAllActorsOfClass` "/Game/Blueprints/Camera/Camera/Level1/EndCamera.EndCamera_C"))
      (set `/Game/Blueprints/Camera/Camera/Level1/EndCamera.CanMove` true (`|GetArrayItem` _outactors_2)))
    (:`B`
      (bind _outactors_3 (`GameplayStatics.GetAllActorsOfClassWithTag` null "Webcam4"))
      (`PlayerController.SetViewTargetWithBlend` (`GameplayStatics.GetPlayerController` 0) (`|GetArrayItem` _outactors_3) 0.0 "VTBlend_Linear" 0.0 false)
      (bind _outactors_4 (`GameplayStatics.GetAllActorsOfClass` "/Game/Blueprints/Camera/Camera/Level1/EndCamera.EndCamera_C"))
      (set `/Game/Blueprints/Camera/Camera/Level1/EndCamera.CanMove` false (`|GetArrayItem` _outactors_4)))))

(fn `UserConstructionScript`)