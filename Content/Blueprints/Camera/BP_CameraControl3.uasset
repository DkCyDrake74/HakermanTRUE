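; Camera controller that pans the BP_Camera_3 cameras and BP_DroneLvl3 with mouse X while the player character's UI is inactive.
; Ten camera classes are found by tag on each input and yawed by clamped input, gated by per-camera angle checks.
; Cam2's checks read this actor's yaw instead of the camera's.
; Lookups nest inside the previous camera's loop, so later cameras and the unclamped drone turn depend on every earlier one existing.
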(event `InputAxisKey|MouseX` :consume false
  (params (AxisValue :type "Float (single-precision)"))
  (bind _returnvalue (`KismetMathLibrary.FClamp` AxisValue -20.0 20.0))
  (bind _returnvalue_2 (`KismetMathLibrary.FClamp` AxisValue -20.0 20.0))
  (bind _returnvalue_3 (`KismetMathLibrary.FClamp` AxisValue -20.0 20.0))
  (bind _returnvalue_4 (`KismetMathLibrary.FClamp` AxisValue -20.0 20.0))
  (bind _returnvalue_5 (`KismetMathLibrary.FClamp` AxisValue -20.0 20.0))
  (bind (_returnvalue_roll _returnvalue_pitch _returnvalue_yaw) (`KismetMathLibrary.BreakRotator` (`self.K2_GetActorRotation`)))
  (bind _returnvalue_6 (`KismetMathLibrary.FClamp` AxisValue -20.0 20.0))
  (bind _returnvalue_7 (`KismetMathLibrary.FClamp` AxisValue -20.0 20.0))
  (bind _returnvalue_8 (`KismetMathLibrary.FClamp` AxisValue -20.0 20.0))
  (bind _returnvalue_9 (`KismetMathLibrary.FClamp` AxisValue -20.0 20.0))
  (bind _returnvalue_10 (`KismetMathLibrary.FClamp` AxisValue -20.0 20.0))
  (bind _asbp_third_person_character (cast `/Game/ThirdPerson/Blueprints/BP_ThirdPersonCharacter` (`GameplayStatics.GetPlayerCharacter` 0)))
  (if (not (`/Game/ThirdPerson/Blueprints/BP_ThirdPersonCharacter.UiIsActive` _asbp_third_person_character))
    (bind _outactors (`GameplayStatics.GetAllActorsOfClassWithTag` "/Game/Blueprints/Camera/Camera/Level3/Camera_Level_3/BP_Camera_3_1.BP_Camera_3_1_C" "Cam1"))
    (for _array_element _outactors
      (bind (_returnvalue_roll_2 _returnvalue_pitch_2 _returnvalue_yaw_2) (`KismetMathLibrary.BreakRotator` (`self.K2_GetActorRotation` _array_element)))
      (bind _output_get (set `self.rotationValidMax` (< _returnvalue_yaw_2 180.0)))
      (bind _output_get_2 (set `self.rotationValidMin` (> _returnvalue_yaw_2 0.0)))
      (bind _rootcomponent (`Actor.RootComponent` _array_element))
      (bind (_returnvalue_roll_3 _returnvalue_pitch_3 _returnvalue_yaw_3) (`KismetMathLibrary.BreakRotator` (`KismetMathLibrary.SelectRotator` (`KismetMathLibrary.MakeRotator` 0.0 0.0 (`KismetMathLibrary.SelectFloat` _returnvalue_5 0.0 _output_get)) (`KismetMathLibrary.MakeRotator` 0.0) true)))
      (`SceneComponent.K2_AddRelativeRotation` _rootcomponent (`KismetMathLibrary.MakeRotator` 0.0 0.0 _returnvalue_yaw_3) false false)
      (bind (_returnvalue_roll_4 _returnvalue_pitch_4 _returnvalue_yaw_4) (`KismetMathLibrary.BreakRotator` (`KismetMathLibrary.SelectRotator` (`KismetMathLibrary.MakeRotator` 0.0) (`KismetMathLibrary.MakeRotator` 0.0 0.0 (`KismetMathLibrary.SelectFloat` _returnvalue_5 0.0 _output_get_2)))))
      (`SceneComponent.K2_AddRelativeRotation` _rootcomponent (`KismetMathLibrary.MakeRotator` 0.0 0.0 _returnvalue_yaw_4) false false)
      (bind _outactors_2 (`GameplayStatics.GetAllActorsOfClassWithTag` "/Game/Blueprints/Camera/Camera/Level3/Camera_Level_3/BP_Camera_3_2.BP_Camera_3_2_C" "Cam2"))
      (for _array_element_2 _outactors_2
        (bind _output_get_3 (set `self.rotationValidMin2` (< _returnvalue_yaw 30.0)))
        (bind _output_get_4 (set `self.rotationValidMax2` (> _returnvalue_yaw -90.0)))
        (bind _rootcomponent_2 (`Actor.RootComponent` _array_element_2))
        (bind (_returnvalue_roll_5 _returnvalue_pitch_5 _returnvalue_yaw_5) (`KismetMathLibrary.BreakRotator` (`KismetMathLibrary.SelectRotator` (`KismetMathLibrary.MakeRotator` 0.0 0.0 (`KismetMathLibrary.SelectFloat` _returnvalue_6 0.0 _output_get_3)) (`KismetMathLibrary.MakeRotator` 0.0) true)))
        (`SceneComponent.K2_AddRelativeRotation` _rootcomponent_2 (`KismetMathLibrary.MakeRotator` 0.0 0.0 _returnvalue_yaw_5) false false)
        (bind (_returnvalue_roll_6 _returnvalue_pitch_6 _returnvalue_yaw_6) (`KismetMathLibrary.BreakRotator` (`KismetMathLibrary.SelectRotator` (`KismetMathLibrary.MakeRotator` 0.0) (`KismetMathLibrary.MakeRotator` 0.0 0.0 (`KismetMathLibrary.SelectFloat` _returnvalue_6 0.0 _output_get_4)))))
        (`SceneComponent.K2_AddRelativeRotation` _rootcomponent_2 (`KismetMathLibrary.MakeRotator` 0.0 0.0 _returnvalue_yaw_6) false false)
        (bind _outactors_3 (`GameplayStatics.GetAllActorsOfClassWithTag` "/Game/Blueprints/Camera/Camera/Level3/Camera_Level_3/BP_Camera_3_3.BP_Camera_3_3_C" "Cam3"))
        (for _array_element_3 _outactors_3
          (bind (_returnvalue_roll_7 _returnvalue_pitch_7 _returnvalue_yaw_7) (`KismetMathLibrary.BreakRotator` (`self.K2_GetActorRotation` _array_element_3)))
          (bind _output_get_5 (set `self.rotationValidMin3` (> _returnvalue_yaw_7 -170.0)))
          (bind _output_get_6 (set `self.rotationValidMax3` (< _returnvalue_yaw_7 -90.0)))
          (bind _rootcomponent_3 (`Actor.RootComponent` _array_element_3))
          (bind (_returnvalue_roll_8 _returnvalue_pitch_8 _returnvalue_yaw_8) (`KismetMathLibrary.BreakRotator` (`KismetMathLibrary.SelectRotator` (`KismetMathLibrary.MakeRotator` 0.0 0.0 (`KismetMathLibrary.SelectFloat` _returnvalue_8 0.0 _output_get_5)) (`KismetMathLibrary.MakeRotator` 0.0) true)))
          (`SceneComponent.K2_AddRelativeRotation` _rootcomponent_3 (`KismetMathLibrary.MakeRotator` 0.0 0.0 _returnvalue_yaw_8) false false)
          (bind (_returnvalue_roll_9 _returnvalue_pitch_9 _returnvalue_yaw_9) (`KismetMathLibrary.BreakRotator` (`KismetMathLibrary.SelectRotator` (`KismetMathLibrary.MakeRotator` 0.0 0.0 (`KismetMathLibrary.SelectFloat` _returnvalue_8 0.0 _output_get_6)) (`KismetMathLibrary.MakeRotator` 0.0) true)))
          (`SceneComponent.K2_AddRelativeRotation` _rootcomponent_3 (`KismetMathLibrary.MakeRotator` 0.0 0.0 _returnvalue_yaw_9) false false)
          (bind _outactors_4 (`GameplayStatics.GetAllActorsOfClassWithTag` "/Game/Blueprints/Camera/Camera/Level3/Camera_Level_3/BP_Camera_3_4.BP_Camera_3_4_C" "Cam4"))
          (for _array_element_4 _outactors_4
            (bind (_returnvalue_roll_10 _returnvalue_pitch_10 _returnvalue_yaw_10) (`KismetMathLibrary.BreakRotator` (`self.K2_GetActorRotation` _array_element_4)))
            (bind _output_get_7 (set `self.rotationValidMin4` (< _returnvalue_yaw_10 170.0)))
            (bind _output_get_8 (set `self.rotationValidMax4` (> _returnvalue_yaw_10 80.0)))
            (bind _rootcomponent_4 (`Actor.RootComponent` _array_element_4))
            (bind (_returnvalue_roll_11 _returnvalue_pitch_11 _returnvalue_yaw_11) (`KismetMathLibrary.BreakRotator` (`KismetMathLibrary.SelectRotator` (`KismetMathLibrary.MakeRotator` 0.0 0.0 (`KismetMathLibrary.SelectFloat` _returnvalue_9 0.0 _output_get_7)) (`KismetMathLibrary.MakeRotator` 0.0) true)))
            (`SceneComponent.K2_AddRelativeRotation` _rootcomponent_4 (`KismetMathLibrary.MakeRotator` 0.0 0.0 _returnvalue_yaw_11) false false)
            (bind (_returnvalue_roll_12 _returnvalue_pitch_12 _returnvalue_yaw_12) (`KismetMathLibrary.BreakRotator` (`KismetMathLibrary.SelectRotator` (`KismetMathLibrary.MakeRotator` 0.0) (`KismetMathLibrary.MakeRotator` 0.0 0.0 (`KismetMathLibrary.SelectFloat` _returnvalue_9 0.0 _output_get_8)))))
            (`SceneComponent.K2_AddRelativeRotation` _rootcomponent_4 (`KismetMathLibrary.MakeRotator` 0.0 0.0 _returnvalue_yaw_12) false false)
            (bind _outactors_5 (`GameplayStatics.GetAllActorsOfClassWithTag` "/Game/Blueprints/Camera/Camera/Level3/Camera_Level_3/BP_Camera_3_5.BP_Camera_3_5_C" "Cam5"))
            (for _array_element_5 _outactors_5
              (bind (_returnvalue_roll_13 _returnvalue_pitch_13 _returnvalue_yaw_13) (`KismetMathLibrary.BreakRotator` (`self.K2_GetActorRotation` _array_element_5)))
              (bind _output_get_9 (set `self.rotationValidMin4` (< _returnvalue_yaw_13 170.0)))
              (bind _output_get_10 (set `self.rotationValidMax4` (> _returnvalue_yaw_13 80.0)))
              (bind _rootcomponent_5 (`Actor.RootComponent` _array_element_5))
              (bind (_returnvalue_roll_14 _returnvalue_pitch_14 _returnvalue_yaw_14) (`KismetMathLibrary.BreakRotator` (`KismetMathLibrary.SelectRotator` (`KismetMathLibrary.MakeRotator` 0.0 0.0 (`KismetMathLibrary.SelectFloat` _returnvalue_10 0.0 _output_get_9)) (`KismetMathLibrary.MakeRotator` 0.0) true)))
              (`SceneComponent.K2_AddRelativeRotation` _rootcomponent_5 (`KismetMathLibrary.MakeRotator` 0.0 0.0 _returnvalue_yaw_14) false false)
              (bind (_returnvalue_roll_15 _returnvalue_pitch_15 _returnvalue_yaw_15) (`KismetMathLibrary.BreakRotator` (`KismetMathLibrary.SelectRotator` (`KismetMathLibrary.MakeRotator` 0.0) (`KismetMathLibrary.MakeRotator` 0.0 0.0 (`KismetMathLibrary.SelectFloat` _returnvalue_10 0.0 _output_get_10)))))
              (`SceneComponent.K2_AddRelativeRotation` _rootcomponent_5 (`KismetMathLibrary.MakeRotator` 0.0 0.0 _returnvalue_yaw_15) false false)
              (bind _outactors_6 (`GameplayStatics.GetAllActorsOfClassWithTag` "/Game/Blueprints/Camera/Camera/Level3/Camera_Level_3/BP_Camera_3_6.BP_Camera_3_6_C" "Cam6"))
              (for _array_element_6 _outactors_6
                (bind (_returnvalue_roll_16 _returnvalue_pitch_16 _returnvalue_yaw_16) (`KismetMathLibrary.BreakRotator` (`self.K2_GetActorRotation` _array_element_6)))
                (bind _output_get_11 (set `self.rotationValidMin4` (< _returnvalue_yaw_16 170.0)))
                (bind _output_get_12 (set `self.rotationValidMax4` (> _returnvalue_yaw_16 80.0)))
                (bind _rootcomponent_6 (`Actor.RootComponent` _array_element_6))
                (bind (_returnvalue_roll_17 _returnvalue_pitch_17 _returnvalue_yaw_17) (`KismetMathLibrary.BreakRotator` (`KismetMathLibrary.SelectRotator` (`KismetMathLibrary.MakeRotator` 0.0 0.0 (`KismetMathLibrary.SelectFloat` _returnvalue 0.0 _output_get_11)) (`KismetMathLibrary.MakeRotator` 0.0) true)))
                (`SceneComponent.K2_AddRelativeRotation` _rootcomponent_6 (`KismetMathLibrary.MakeRotator` 0.0 0.0 _returnvalue_yaw_17) false false)
                (bind (_returnvalue_roll_18 _returnvalue_pitch_18 _returnvalue_yaw_18) (`KismetMathLibrary.BreakRotator` (`KismetMathLibrary.SelectRotator` (`KismetMathLibrary.MakeRotator` 0.0) (`KismetMathLibrary.MakeRotator` 0.0 0.0 (`KismetMathLibrary.SelectFloat` _returnvalue 0.0 _output_get_12)))))
                (`SceneComponent.K2_AddRelativeRotation` _rootcomponent_6 (`KismetMathLibrary.MakeRotator` 0.0 0.0 _returnvalue_yaw_18) false false)
                (bind _outactors_7 (`GameplayStatics.GetAllActorsOfClassWithTag` "/Game/Blueprints/Camera/Camera/Level3/Camera_Level_3/BP_Camera_3_7.BP_Camera_3_7_C" "Cam7"))
                (for _array_element_7 _outactors_7
                  (bind (_returnvalue_roll_19 _returnvalue_pitch_19 _returnvalue_yaw_19) (`KismetMathLibrary.BreakRotator` (`self.K2_GetActorRotation` _array_element_7)))
                  (bind _output_get_13 (set `self.rotationValidMin4` (< _returnvalue_yaw_19 0.0)))
                  (bind _output_get_14 (set `self.rotationValidMax4` (> _returnvalue_yaw_19 0.0)))
                  (bind _rootcomponent_7 (`Actor.RootComponent` _array_element_7))
                  (bind (_returnvalue_roll_20 _returnvalue_pitch_20 _returnvalue_yaw_20) (`KismetMathLibrary.BreakRotator` (`KismetMathLibrary.SelectRotator` (`KismetMathLibrary.MakeRotator` 0.0 0.0 (`KismetMathLibrary.SelectFloat` _returnvalue_2 0.0 _output_get_13)) (`KismetMathLibrary.MakeRotator` 0.0) true)))
                  (`SceneComponent.K2_AddRelativeRotation` _rootcomponent_7 (`KismetMathLibrary.MakeRotator` 0.0 0.0 _returnvalue_yaw_20) false false)
                  (bind (_returnvalue_roll_21 _returnvalue_pitch_21 _returnvalue_yaw_21) (`KismetMathLibrary.BreakRotator` (`KismetMathLibrary.SelectRotator` (`KismetMathLibrary.MakeRotator` 0.0) (`KismetMathLibrary.MakeRotator` 0.0 0.0 (`KismetMathLibrary.SelectFloat` _returnvalue_2 0.0 _output_get_14)))))
                  (`SceneComponent.K2_AddRelativeRotation` _rootcomponent_7 (`KismetMathLibrary.MakeRotator` 0.0 0.0 _returnvalue_yaw_21) false false)
                  (bind _outactors_8 (`GameplayStatics.GetAllActorsOfClassWithTag` "/Game/Blueprints/Camera/Camera/Level3/Camera_Level_3/BP_Camera_3_8.BP_Camera_3_8_C" "Cam8"))
                  (for _array_element_8 _outactors_8
                    (bind (_returnvalue_roll_22 _returnvalue_pitch_22 _returnvalue_yaw_22) (`KismetMathLibrary.BreakRotator` (`self.K2_GetActorRotation` _array_element_8)))
                    (bind _output_get_15 (set `self.rotationValidMin4` (< _returnvalue_yaw_22 170.0)))
                    (bind _output_get_16 (set `self.rotationValidMax4` (> _returnvalue_yaw_22 80.0)))
                    (bind _rootcomponent_8 (`Actor.RootComponent` _array_element_8))
                    (bind (_returnvalue_roll_23 _returnvalue_pitch_23 _returnvalue_yaw_23) (`KismetMathLibrary.BreakRotator` (`KismetMathLibrary.SelectRotator` (`KismetMathLibrary.MakeRotator` 0.0 0.0 (`KismetMathLibrary.SelectFloat` _returnvalue_3 0.0 _output_get_15)) (`KismetMathLibrary.MakeRotator` 0.0) true)))
                    (`SceneComponent.K2_AddRelativeRotation` _rootcomponent_8 (`KismetMathLibrary.MakeRotator` 0.0 0.0 _returnvalue_yaw_23) false false)
                    (bind (_returnvalue_roll_24 _returnvalue_pitch_24 _returnvalue_yaw_24) (`KismetMathLibrary.BreakRotator` (`KismetMathLibrary.SelectRotator` (`KismetMathLibrary.MakeRotator` 0.0) (`KismetMathLibrary.MakeRotator` 0.0 0.0 (`KismetMathLibrary.SelectFloat` _returnvalue_3 0.0 _output_get_16)))))
                    (`SceneComponent.K2_AddRelativeRotation` _rootcomponent_8 (`KismetMathLibrary.MakeRotator` 0.0 0.0 _returnvalue_yaw_24) false false)
                    (bind _outactors_9 (`GameplayStatics.GetAllActorsOfClassWithTag` "/Game/Blueprints/Camera/Camera/Level3/Camera_Level_3/BP_Camera_3_9.BP_Camera_3_9_C" "Cam9"))
                    (for _array_element_9 _outactors_9
                      (bind (_returnvalue_roll_25 _returnvalue_pitch_25 _returnvalue_yaw_25) (`KismetMathLibrary.BreakRotator` (`self.K2_GetActorRotation` _array_element_9)))
                      (bind _output_get_17 (set `self.rotationValidMin4` (< _returnvalue_yaw_25 170.0)))
                      (bind _output_get_18 (set `self.rotationValidMax4` (> _returnvalue_yaw_25 80.0)))
                      (bind _rootcomponent_9 (`Actor.RootComponent` _array_element_9))
                      (bind (_returnvalue_roll_26 _returnvalue_pitch_26 _returnvalue_yaw_26) (`KismetMathLibrary.BreakRotator` (`KismetMathLibrary.SelectRotator` (`KismetMathLibrary.MakeRotator` 0.0 0.0 (`KismetMathLibrary.SelectFloat` _returnvalue_4 0.0 _output_get_17)) (`KismetMathLibrary.MakeRotator` 0.0) true)))
                      (`SceneComponent.K2_AddRelativeRotation` _rootcomponent_9 (`KismetMathLibrary.MakeRotator` 0.0 0.0 _returnvalue_yaw_26) false false)
                      (bind (_returnvalue_roll_27 _returnvalue_pitch_27 _returnvalue_yaw_27) (`KismetMathLibrary.BreakRotator` (`KismetMathLibrary.SelectRotator` (`KismetMathLibrary.MakeRotator` 0.0) (`KismetMathLibrary.MakeRotator` 0.0 0.0 (`KismetMathLibrary.SelectFloat` _returnvalue_4 0.0 _output_get_18)))))
                      (`SceneComponent.K2_AddRelativeRotation` _rootcomponent_9 (`KismetMathLibrary.MakeRotator` 0.0 0.0 _returnvalue_yaw_27) false false)
                      (bind _outactors_10 (`GameplayStatics.GetAllActorsOfClassWithTag` "/Game/Blueprints/Camera/Camera/Level3/Camera_Level_3/BP_Camera_3_10.BP_Camera_3_10_C" "Cam10"))
                      (for _array_element_10 _outactors_10
                        (bind (_returnvalue_roll_28 _returnvalue_pitch_28 _returnvalue_yaw_28) (`KismetMathLibrary.BreakRotator` (`self.K2_GetActorRotation` _array_element_10)))
                        (bind _output_get_19 (set `self.rotationValidMin4` (< _returnvalue_yaw_28 170.0)))
                        (bind _output_get_20 (set `self.rotationValidMax4` (> _returnvalue_yaw_28 80.0)))
                        (bind _rootcomponent_10 (`Actor.RootComponent` _array_element_10))
                        (bind (_returnvalue_roll_29 _returnvalue_pitch_29 _returnvalue_yaw_29) (`KismetMathLibrary.BreakRotator` (`KismetMathLibrary.SelectRotator` (`KismetMathLibrary.MakeRotator` 0.0 0.0 (`KismetMathLibrary.SelectFloat` _returnvalue_7 0.0 _output_get_19)) (`KismetMathLibrary.MakeRotator` 0.0) true)))
                        (`SceneComponent.K2_AddRelativeRotation` _rootcomponent_10 (`KismetMathLibrary.MakeRotator` 0.0 0.0 _returnvalue_yaw_29) false false)
                        (bind (_returnvalue_roll_30 _returnvalue_pitch_30 _returnvalue_yaw_30) (`KismetMathLibrary.BreakRotator` (`KismetMathLibrary.SelectRotator` (`KismetMathLibrary.MakeRotator` 0.0) (`KismetMathLibrary.MakeRotator` 0.0 0.0 (`KismetMathLibrary.SelectFloat` _returnvalue_7 0.0 _output_get_20)))))
                        (`SceneComponent.K2_AddRelativeRotation` _rootcomponent_10 (`KismetMathLibrary.MakeRotator` 0.0 0.0 _returnvalue_yaw_30) false false)
                        (bind _outactors_11 (`GameplayStatics.GetAllActorsOfClass` "/Game/Blueprints/Drone/Level3/BP_DroneLvl3.BP_DroneLvl3_C"))
                        (for _array_element_11 _outactors_11
                          (`SceneComponent.K2_AddRelativeRotation` (`Actor.RootComponent` _array_element_11) (`KismetMathLibrary.MakeRotator` 0.0 0.0 AxisValue) false false))))))))))))))

(fn `UserConstructionScript`)