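; BP_Camera_0_1 is a Level0 security camera that supports mouse-driven panning within a yaw range.
; Tick prints the actor's yaw and sets CanRotate only while it lies between MinPos and MaxPos1.
; When CanRotate is true and character UI is inactive, MouseX yaws the current view target's root, not necessarily this actor, excluding the first TrackingCamera0.
; SetRenderCustomDepth toggles custom depth on the camera mesh.
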(event `InputAxisKey|MouseX` :consume false
  (params (AxisValue :type "Float (single-precision)"))
  (bind _returnvalue (`Controller.GetViewTarget` (`GameplayStatics.GetPlayerController` 0)))
  (bind _asbp_third_person_character (cast `/Game/ThirdPerson/Blueprints/BP_ThirdPersonCharacter` (`GameplayStatics.GetPlayerCharacter` 0)))
  (if (`/Game/ThirdPerson/Blueprints/BP_ThirdPersonCharacter.UiIsActive` _asbp_third_person_character)
    _
    (elif (`self.CanRotate`)
      (bind _outactors (`GameplayStatics.GetAllActorsOfClass` "/Game/Blueprints/Camera/Camera/Level1/TrackingCamera0.TrackingCamera0_C"))
      (if (!= _returnvalue (`|GetArrayItem` _outactors))
        (`SceneComponent.K2_AddRelativeRotation` (`Actor.RootComponent` _returnvalue) (`KismetMathLibrary.MakeRotator` 0.0 0.0 AxisValue) false false)))))

(event `self.ReceiveTick`
  (params (DeltaSeconds :type "Float (single-precision)"))
  (bind (_returnvalue_roll _returnvalue_pitch _returnvalue_yaw) (`KismetMathLibrary.BreakRotator` (`self.K2_GetActorRotation`)))
  (`KismetSystemLibrary.PrintString` (`KismetStringLibrary.Conv_DoubleToString` _returnvalue_yaw) true true (struct :`G` 0.66 :`B` 1.0 :`A` 1.0) 0.01)
  (if (and (>= _returnvalue_yaw (`self.MinPos`)) (<= _returnvalue_yaw (`self.MaxPos1`)))
    (set `self.CanRotate` true)
    (else
      (set `self.CanRotate` false))))

(fn `SetRenderCustomDepth`
  (params (RenderCustomDepth :type Boolean))
  (`PrimitiveComponent.SetRenderCustomDepth` (`self.SM_SecurityCameraSet02`) RenderCustomDepth))

(fn `UserConstructionScript`)