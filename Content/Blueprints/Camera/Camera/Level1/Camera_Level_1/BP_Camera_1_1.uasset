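; BP_Camera_1_1 is a Level 1 camera that the player can turn horizontally with the mouse.
; The MouseX axis event adds yaw to its root component while it is the player controller's view target.
; Rotation is skipped when the third-person character's UiIsActive flag is set or the player pawn is not a BP_ThirdPersonCharacter.
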(event `InputAxisKey|MouseX` :consume false
  (params (AxisValue :type "Float (single-precision)"))
  (bind _returnvalue (`Controller.GetViewTarget` (`GameplayStatics.GetPlayerController` 0)))
  (bind _asbp_third_person_character (cast `/Game/ThirdPerson/Blueprints/BP_ThirdPersonCharacter` (`GameplayStatics.GetPlayerCharacter` 0)))
  (if (`/Game/ThirdPerson/Blueprints/BP_ThirdPersonCharacter.UiIsActive` _asbp_third_person_character)
    _
    (elif (== _returnvalue self)
      (`SceneComponent.K2_AddRelativeRotation` (`Actor.RootComponent` _returnvalue) (`KismetMathLibrary.MakeRotator` 0.0 0.0 AxisValue) false false))))

(fn `UserConstructionScript`)