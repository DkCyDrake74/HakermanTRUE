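; BP_Start_Camera is a trigger actor that switches the player's view between two cameras on entering its Box component.
; Each overlap advances a FlipFlop: the first blends the view to the StartCamera actor and enables its CanMove flag.
; The next blends to the CameraActor tagged Start_Camera and disables CanMove.
; Targets are found at runtime by class or tag lookup, and the overlapping actor is not checked.
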(event `self.Box.OnComponentBeginOverlap`
  (params (OverlappedComponent :type "PrimitiveComponent Object Reference") (OtherActor :type "Actor Object Reference") (OtherComp :type "PrimitiveComponent Object Reference") (OtherBodyIndex :type Integer) (bFromSweep :type Boolean) (SweepResult :type "HitResult Structure (by ref)"))
  (`/Engine/EditorBlueprintResources/StandardMacros.FlipFlop`
    (:`A`
      (bind _outactors (`GameplayStatics.GetAllActorsOfClass` "/Game/Blueprints/Camera/Camera/Level1/StartCamera.StartCamera_C"))
      (`PlayerController.SetViewTargetWithBlend` (`GameplayStatics.GetPlayerController` 0) (`|GetArrayItem` _outactors) 0.0 "VTBlend_Linear" 0.0 false)
      (bind _returnvalue (`GameplayStatics.GetActorOfClass` "/Game/Blueprints/Camera/Camera/Level1/StartCamera.StartCamera_C"))
      (set `/Game/Blueprints/Camera/Camera/Level1/StartCamera.CanMove` true _returnvalue))
    (:`B`
      (bind _outactors_2 (`GameplayStatics.GetAllActorsOfClassWithTag` "/Script/Engine.CameraActor" "Start_Camera"))
      (`PlayerController.SetViewTargetWithBlend` (`GameplayStatics.GetPlayerController` 0) (`|GetArrayItem` _outactors_2) 0.0 "VTBlend_Linear" 0.0 false)
      (bind _returnvalue_2 (`GameplayStatics.GetActorOfClass` "/Game/Blueprints/Camera/Camera/Level1/StartCamera.StartCamera_C"))
      (set `/Game/Blueprints/Camera/Camera/Level1/StartCamera.CanMove` false _returnvalue_2))))

(fn `UserConstructionScript`)