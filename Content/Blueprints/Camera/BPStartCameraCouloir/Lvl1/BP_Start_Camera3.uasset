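; BP_Start_Camera3 is a level 1 trigger box that switches the player's view to a corridor camera.
; When the third-person character overlaps it, the view target becomes the BP_Camera_1_1 tagged Cam1, the TrackingCamera stops moving, and a WD_HUD widget is added.
; It also sets the character's active camera index to 1, then starts the first-side scan on BP_DIversionScanLevel1.
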(event `self.Box.OnComponentBeginOverlap`
  (params (OverlappedComponent :type "PrimitiveComponent Object Reference") (OtherActor :type "Actor Object Reference") (OtherComp :type "PrimitiveComponent Object Reference") (OtherBodyIndex :type Integer) (bFromSweep :type Boolean) (SweepResult :type "HitResult Structure (by ref)"))
  (cast `/Game/ThirdPerson/Blueprints/BP_ThirdPersonCharacter` OtherActor)
  (`|ExecutionSequence`
    (:`then_0`
      (bind _outactors (`GameplayStatics.GetAllActorsOfClassWithTag` "/Game/Blueprints/Camera/Camera/Level1/Camera_Level_1/BP_Camera_1_1.BP_Camera_1_1_C" "Cam1"))
      (`PlayerController.SetViewTargetWithBlend` (`GameplayStatics.GetPlayerController` 0) (`|GetArrayItem` _outactors) 0.0 "VTBlend_Linear" 0.0 false)
      (bind _outactors_2 (`GameplayStatics.GetAllActorsOfClass` "/Game/Blueprints/Camera/Camera/Level1/TrackingCamera.TrackingCamera_C"))
      (set `/Game/Blueprints/Camera/Camera/Level1/TrackingCamera.CanMove` false (`|GetArrayItem` _outactors_2))
      (bind _returnvalue (`|CreateWidget` "/Game/UI/HUD/WD_HUD.WD_HUD_C"))
      (`UserWidget.AddToViewport` _returnvalue 0)
      (bind _asbp_third_person_character (cast `/Game/ThirdPerson/Blueprints/BP_ThirdPersonCharacter` (`GameplayStatics.GetPlayerCharacter` 0)))
      (set `/Game/ThirdPerson/Blueprints/BP_ThirdPersonCharacter.getActiveCamera1` 1 _asbp_third_person_character))
    (:`then_1`
      (bind _outactors_3 (`GameplayStatics.GetAllActorsOfClass` "/Game/PostProcess/BP_DIversionScanLevel1.BP_DIversionScanLevel1_C"))
      (`/Game/PostProcess/BP_DIversionScanLevel1.ScanFirstSide` (`|GetArrayItem` _outactors_3)))))

(fn `UserConstructionScript`)