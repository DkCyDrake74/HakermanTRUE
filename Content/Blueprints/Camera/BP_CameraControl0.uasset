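; BP_CameraControl0 lets horizontal mouse input yaw the player's current camera view target while CanRotate is set and the third-person character's UI is inactive.
; On each MouseX event it loops over BP_Camera_0_1 actors tagged "Camera", skipping rotation if the view target is the first TrackingCamera0.
; For each camera with world yaw inside ±90 degrees, it prints that yaw and rotates the view target's root component, not the looped camera.
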(event `InputAxisKey|MouseX` :consume false
  (params (AxisValue :type "Float (single-precision)"))
  (bind _returnvalue (`Controller.GetViewTarget` (`GameplayStatics.GetPlayerController` 0)))
  (bind _asbp_third_person_character (cast `/Game/ThirdPerson/Blueprints/BP_ThirdPersonCharacter` (`GameplayStatics.GetPlayerCharacter` 0)))
  (if (`/Game/ThirdPerson/Blueprints/BP_ThirdPersonCharacter.UiIsActive` _asbp_third_person_character)
    _
    (elif (`self.CanRotate`)
      (bind _outactors (`GameplayStatics.GetAllActorsOfClassWithTag` "/Game/Blueprints/Camera/Camera/Level0/BP_Camera_0_1.BP_Camera_0_1_C" "Camera"))
      (for _array_element _outactors
        (bind _outactors_2 (`GameplayStatics.GetAllActorsOfClass` "/Game/Blueprints/Camera/Camera/Level1/TrackingCamera0.TrackingCamera0_C"))
        (bind (_returnvalue_roll _returnvalue_pitch _returnvalue_yaw) (`KismetMathLibrary.BreakRotator` (`self.K2_GetActorRotation` _array_element)))
        (if (and (!= _returnvalue (`|GetArrayItem` _outactors_2)) (and (< _returnvalue_yaw 90.0) (> _returnvalue_yaw -90.0)))
          (`KismetSystemLibrary.PrintString` (`KismetStringLibrary.Conv_DoubleToString` _returnvalue_yaw))
          (`SceneComponent.K2_AddRelativeRotation` (`Actor.RootComponent` _returnvalue) (`KismetMathLibrary.MakeRotator` 0.0 0.0 AxisValue) false false))))))

(fn `UserConstructionScript`)