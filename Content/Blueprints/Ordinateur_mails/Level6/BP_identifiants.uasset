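; BP_identifiants is an interactable credentials note that the player picks up to add to the Néo Z.
; Box overlap by the third-person character highlights the cube through custom depth, shows the Widget component, enables input and flags the character's UI active.
; Interact, through a DoOnce, plays a sound, displays WD_Identifiants and briefly shows a WD_Aide pickup message.
; Leaving the box reverses the overlap state and removes the credentials widget.
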(event `InputAction|Interact`
  (params (Key :type "Key Structure"))
  (:`Pressed`
    (if (`self.CanOpen?`)
      (set `self.IsOpen` true)
      (`/Engine/EditorBlueprintResources/StandardMacros.DoOnce` false
        (:`Completed`
          (`GameplayStatics.PlaySound2D` "/Game/Sound/SFX/Enigme/Validation_enigma.Validation_enigma" 1.0 1.0 0.0 null null)
          (bind _returnvalue (`|CreateWidget` "/Game/UI/Ordinateurs/Level1/WD_Identifiants.WD_Identifiants_C"))
          (`UserWidget.AddToViewport` _returnvalue 0)
          (`KismetSystemLibrary.Delay` 0.5)
          (bind _foundwidgets (`WidgetBlueprintLibrary.GetAllWidgetsOfClass` "/Game/UI/WD_Aide.WD_Aide_C"))
          (bind _texteaide1 (`/Game/UI/WD_Aide.TexteAide1` (`|GetArrayItem` _foundwidgets)))
          (`TextBlock.SetText` _texteaide1 "NOTE RÉCUPÉRER ET AJOUTÉ AU NÉO Z")
          (`Widget.SetVisibility` _texteaide1 "Visible")
          (`KismetSystemLibrary.Delay` 3.0)
          (`Widget.SetVisibility` _texteaide1 "Hidden"))))))

(event `self.Box.OnComponentBeginOverlap`
  (params (OverlappedComponent :type "PrimitiveComponent Object Reference") (OtherActor :type "Actor Object Reference") (OtherComp :type "PrimitiveComponent Object Reference") (OtherBodyIndex :type Integer) (bFromSweep :type Boolean) (SweepResult :type "HitResult Structure (by ref)"))
  (cast `/Game/ThirdPerson/Blueprints/BP_ThirdPersonCharacter` OtherActor)
  (`PrimitiveComponent.SetRenderCustomDepth` (`self.Cube`) true)
  (`|ExecutionSequence`
    (:`then_0`
      (cast `/Game/ThirdPerson/Blueprints/BP_ThirdPersonCharacter` OtherActor)
      (`self.EnableInput` (`GameplayStatics.GetPlayerController` 0))
      (set `self.CanOpen?` true)
      (bind _asbp_third_person_character (cast `/Game/ThirdPerson/Blueprints/BP_ThirdPersonCharacter` (`GameplayStatics.GetPlayerCharacter` 0)))
      (set `/Game/ThirdPerson/Blueprints/BP_ThirdPersonCharacter.UiIsActive` true _asbp_third_person_character))
    (:`then_1`
      (set `self.CanSee?` true)
      (`SceneComponent.SetVisibility` (`self.Widget`) true false))))

(event `self.Box.OnComponentEndOverlap`
  (params (OverlappedComponent :type "PrimitiveComponent Object Reference") (OtherActor :type "Actor Object Reference") (OtherComp :type "PrimitiveComponent Object Reference") (OtherBodyIndex :type Integer))
  (cast `/Game/ThirdPerson/Blueprints/BP_ThirdPersonCharacter` OtherActor)
  (`PrimitiveComponent.SetRenderCustomDepth` (`self.Cube`) false)
  (`|ExecutionSequence`
    (:`then_0`
      (cast `/Game/ThirdPerson/Blueprints/BP_ThirdPersonCharacter` OtherActor)
      (`self.DisableInput` (`GameplayStatics.GetPlayerController` 0))
      (set `self.CanOpen?` false)
      (bind _asbp_third_person_character (cast `/Game/ThirdPerson/Blueprints/BP_ThirdPersonCharacter` (`GameplayStatics.GetPlayerCharacter` 0)))
      (set `/Game/ThirdPerson/Blueprints/BP_ThirdPersonCharacter.UiIsActive` false _asbp_third_person_character)
      (if (`self.IsOpen`)
        (`Widget.RemoveFromParent` (stale `InputAction|Interact` _returnvalue))
        (set `self.IsOpen` false)))
    (:`then_1`
      (set `self.CanSee?` false)
      (`SceneComponent.SetVisibility` (`self.Widget`) false false))))

(fn `UserConstructionScript`)