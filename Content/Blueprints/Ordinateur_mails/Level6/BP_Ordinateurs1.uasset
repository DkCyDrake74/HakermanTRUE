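; Interactable computer that opens the WD_Ordinateur screen with a mouse cursor when the player presses Interact nearby.
; A Box overlap by the third-person character enables input and CanOpen, while any overlap shows the Widget component.
; On end overlap, the character loses input and open computer or mail login screens are removed along with the cursor.
; The Widget component hides when any actor leaves the box.
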(event `InputAction|Interact`
  (params (Key :type "Key Structure"))
  (:`Pressed`
    (if (`self.CanOpen`)
      (bind _returnvalue (`|CreateWidget` "/Game/UI/Ordinateurs/Level1/WD_Ordinateur.WD_Ordinateur_C"))
      (`UserWidget.AddToViewport` _returnvalue 0)
      (set `PlayerController.bShowMouseCursor` true (`GameplayStatics.GetPlayerController` 0)))))

(event `self.Box.OnComponentBeginOverlap`
  (params (OverlappedComponent :type "PrimitiveComponent Object Reference") (OtherActor :type "Actor Object Reference") (OtherComp :type "PrimitiveComponent Object Reference") (OtherBodyIndex :type Integer) (bFromSweep :type Boolean) (SweepResult :type "HitResult Structure (by ref)"))
  (`|ExecutionSequence`
    (:`then_0`
      (cast `/Game/ThirdPerson/Blueprints/BP_ThirdPersonCharacter` OtherActor)
      (`self.EnableInput` (`GameplayStatics.GetPlayerController` 0))
      (set `self.CanOpen` true))
    (:`then_1`
      (set `self.CanSee?` true)
      (`SceneComponent.SetVisibility` (`self.Widget`) true false))))

(event `self.Box.OnComponentEndOverlap`
  (params (OverlappedComponent :type "PrimitiveComponent Object Reference") (OtherActor :type "Actor Object Reference") (OtherComp :type "PrimitiveComponent Object Reference") (OtherBodyIndex :type Integer))
  (`|ExecutionSequence`
    (:`then_0`
      (cast `/Game/ThirdPerson/Blueprints/BP_ThirdPersonCharacter` OtherActor)
      (`self.DisableInput` (`GameplayStatics.GetPlayerController` 0))
      (set `self.CanOpen` false)
      (`|ExecutionSequence`
        (:`then_0`
          (`/Engine/EditorBlueprintResources/StandardMacros.IsValid` "/Game/UI/Ordinateurs/Level1/WD_Ordinateur.WD_Ordinateur"
            (:`Is Valid`
              (bind _foundwidgets (`WidgetBlueprintLibrary.GetAllWidgetsOfClass` "/Game/UI/Ordinateurs/Level1/WD_Ordinateur.WD_Ordinateur_C")))))
        (:`then_1`
          (`/Engine/EditorBlueprintResources/StandardMacros.IsValid` "/Game/UI/Ordinateurs/Level1/WD_Mail_Login.WD_Mail_Login"
            (:`Is Valid`
              (bind _foundwidgets_2 (`WidgetBlueprintLibrary.GetAllWidgetsOfClass` "/Game/UI/Ordinateurs/Level1/WD_Mail_Login.WD_Mail_Login_C")))))
        (:`then_2`
          (`/Engine/EditorBlueprintResources/StandardMacros.IsValid` "/Game/UI/Ordinateurs/Level1/WD_Ordinateur.WD_Ordinateur"
            (:`Is Valid`
              (bind _foundwidgets_3 (`WidgetBlueprintLibrary.GetAllWidgetsOfClass` "/Game/UI/Ordinateurs/Level1/WD_Ordinateur.WD_Ordinateur_C"))))))
      (`Widget.RemoveFromParent` (stale `InputAction|Interact` _returnvalue))
      (`Widget.RemoveFromParent` (`|GetArrayItem` _foundwidgets))
      (`Widget.RemoveFromParent` (`|GetArrayItem` _foundwidgets_2))
      (`Widget.RemoveFromParent` (`|GetArrayItem` _foundwidgets_3))
      (set `PlayerController.bShowMouseCursor` false (`GameplayStatics.GetPlayerController` 0)))
    (:`then_1`
      (set `self.CanSee?` false)
      (`SceneComponent.SetVisibility` (`self.Widget`) false false))))

(fn `UserConstructionScript`)