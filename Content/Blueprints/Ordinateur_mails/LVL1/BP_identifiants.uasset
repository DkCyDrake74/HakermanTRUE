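; Interactable credentials (identifiants) trigger in the LVL1 computer-mail content that shows the WD_Identifiants widget.
; Overlapping its Box with the third-person character enables input, allows opening and sets the character's UiIsActive flag.
; Pressing Interact plays the enigma-validation sound and adds the widget, behind a DoOnce that is never reset.
; Leaving the Box disables input, clears both flags and removes the widget.
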(event `InputAction|Interact`
  (params (Key :type "Key Structure"))
  (:`Pressed`
    (if (`self.CanOpen?`)
      (`/Engine/EditorBlueprintResources/StandardMacros.DoOnce` false
        (:`Completed`
          (`GameplayStatics.PlaySound2D` "/Game/Sound/SFX/Enigme/Validation_enigma.Validation_enigma" 1.0 1.0 0.0 null null)
          (bind _returnvalue (`|CreateWidget` "/Game/UI/Ordinateurs/Level1/WD_Identifiants.WD_Identifiants_C"))
          (`UserWidget.AddToViewport` _returnvalue 0))))))

(event `self.Box.OnComponentBeginOverlap`
  (params (OverlappedComponent :type "PrimitiveComponent Object Reference") (OtherActor :type "Actor Object Reference") (OtherComp :type "PrimitiveComponent Object Reference") (OtherBodyIndex :type Integer) (bFromSweep :type Boolean) (SweepResult :type "HitResult Structure (by ref)"))
  (cast `/Game/ThirdPerson/Blueprints/BP_ThirdPersonCharacter` OtherActor)
  (`self.EnableInput` (`GameplayStatics.GetPlayerController` 0))
  (set `self.CanOpen?` true)
  (bind _asbp_third_person_character (cast `/Game/ThirdPerson/Blueprints/BP_ThirdPersonCharacter` (`GameplayStatics.GetPlayerCharacter` 0)))
  (set `/Game/ThirdPerson/Blueprints/BP_ThirdPersonCharacter.UiIsActive` true _asbp_third_person_character))

(event `self.Box.OnComponentEndOverlap`
  (params (OverlappedComponent :type "PrimitiveComponent Object Reference") (OtherActor :type "Actor Object Reference") (OtherComp :type "PrimitiveComponent Object Reference") (OtherBodyIndex :type Integer))
  (cast `/Game/ThirdPerson/Blueprints/BP_ThirdPersonCharacter` OtherActor)
  (`self.DisableInput` (`GameplayStatics.GetPlayerController` 0))
  (set `self.CanOpen?` false)
  (bind _asbp_third_person_character (cast `/Game/ThirdPerson/Blueprints/BP_ThirdPersonCharacter` (`GameplayStatics.GetPlayerCharacter` 0)))
  (set `/Game/ThirdPerson/Blueprints/BP_ThirdPersonCharacter.UiIsActive` false _asbp_third_person_character)
  (`Widget.RemoveFromParent` (stale `InputAction|Interact` _returnvalue)))

(fn `UserConstructionScript`)