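; BP_identifiants is a trigger that reveals email login credentials, likely for a computer mail puzzle.
; Overlapping its Box creates and displays a WD_Identifiants widget, then writes the hardcoded login and password into the player character's NotesIdentifiants.
; It prints that note immediately and again after a short delay.
; Ending the overlap removes the widget; neither overlap event checks which actor triggered it.
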(event `self.Box.OnComponentBeginOverlap`
  (params (OverlappedComponent :type "PrimitiveComponent Object Reference") (OtherActor :type "Actor Object Reference") (OtherComp :type "PrimitiveComponent Object Reference") (OtherBodyIndex :type Integer) (bFromSweep :type Boolean) (SweepResult :type "HitResult Structure (by ref)"))
  (bind _returnvalue (`|CreateWidget` "/Game/UI/Ordinateurs/WD_Identifiants.WD_Identifiants_C"))
  (bind _output_get (set `self.WD_Identifiants_Ref` _returnvalue))
  (`UserWidget.AddToViewport` _output_get 0)
  (bind _asbp_third_person_character (cast `/Game/ThirdPerson/Blueprints/BP_ThirdPersonCharacter` (`GameplayStatics.GetPlayerCharacter` 0)))
  (bind _output_get_2 (set `/Game/ThirdPerson/Blueprints/BP_ThirdPersonCharacter.Notes_Identifiants` "Login : evilcorp@jmail.com \nPassword : evilcorp" _asbp_third_person_character))
  (`KismetSystemLibrary.PrintText` _output_get_2)
  (`KismetSystemLibrary.Delay` 5.0)
  (`KismetSystemLibrary.PrintText` _output_get_2))

(event `self.Box.OnComponentEndOverlap`
  (params (OverlappedComponent :type "PrimitiveComponent Object Reference") (OtherActor :type "Actor Object Reference") (OtherComp :type "PrimitiveComponent Object Reference") (OtherBodyIndex :type Integer))
  (`Widget.RemoveFromParent` (stale `self.Box.OnComponentBeginOverlap` _output_get)))

(fn `UserConstructionScript`)