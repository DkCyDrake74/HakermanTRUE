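; Interactable door for level 1 that swings open and closed on Interact, but only once its RouterIsOk flag is true.
; A box overlap enables player input and shows the door's widget, then reverses both on exit.
; A timeline yaws the door mesh from its starting rotation and plays in reverse to close, with open and close sounds.
; While locked, Interact briefly shows a French "door locked" message in the WD_Aide help widget.
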(event `self.ReceiveBeginPlay`
  ;[0 0.05647 1] Init Rotation
  (set `self.RotationDepart` (`SceneComponent.RelativeRotation` (`self.Porte`))))

(event `InputAction|Interact`
  (params (Key :type "Key Structure"))
  ;[0.02595 1 0] Open / Close Door
  (:`Pressed`
    (if (`self.RouterIsOk`)
      (if (`self.CanOpen2?`)
        (if (`self.close_Door`)
          (`AudioComponent.Play` (`self.OpenDoor`) 0.0)
          (bind (_direction _rotation) (`Timeline|Timeline` :!label _label)
            (:`Update`
              (`SceneComponent.K2_SetRelativeRotation` (`self.Porte`) (`KismetMathLibrary.MakeRotator` (.roll (`self.RotationDepart`)) (.pitch (`self.RotationDepart`)) (+ _rotation (.yaw (`self.RotationDepart`)))) false false)
              (set `self.close_Door` (< _rotation 1.0))))
          (else
            (`AudioComponent.Play` (`self.CloseDoor`) 0.0)
            (goto _label :!via `Reverse`))))
      (else
        (`KismetSystemLibrary.Delay` 0.5)
        (bind _foundwidgets (`WidgetBlueprintLibrary.GetAllWidgetsOfClass` "/Game/UI/WD_Aide.WD_Aide_C"))
        (bind _texteaide1 (`/Game/UI/WD_Aide.TexteAide1` (`|GetArrayItem` _foundwidgets)))
        (`TextBlock.SetText` _texteaide1 "PORTE VÉRROUILLÉ")
        (`Widget.SetVisibility` _texteaide1 "Visible")
        (`KismetSystemLibrary.Delay` 2.0)
        (`Widget.SetVisibility` _texteaide1 "Hidden")))))

(event `self.Box.OnComponentBeginOverlap`
  (params (OverlappedComponent :type "PrimitiveComponent Object Reference") (OtherActor :type "Actor Object Reference") (OtherComp :type "PrimitiveComponent Object Reference") (OtherBodyIndex :type Integer) (bFromSweep :type Boolean) (SweepResult :type "HitResult Structure (by ref)"))
  (`|ExecutionSequence`
    (:`then_0`
      ;[1 0.9213 0] Enable / Disable input
      (set `self.CanOpen2?` true)
      (cast `/Game/ThirdPerson/Blueprints/BP_ThirdPersonCharacter` (`GameplayStatics.GetPlayerCharacter` 0))
      (cast `/Game/ThirdPerson/Blueprints/BP_ThirdPersonCharacter` OtherActor)
      (`self.EnableInput` (`GameplayStatics.GetPlayerController` 0)))
    (:`then_1`
      (set `self.CanSee?` true)
      (`SceneComponent.SetVisibility` (`self.Widget`) true false))))

(event `self.Box.OnComponentEndOverlap`
  (params (OverlappedComponent :type "PrimitiveComponent Object Reference") (OtherActor :type "Actor Object Reference") (OtherComp :type "PrimitiveComponent Object Reference") (OtherBodyIndex :type Integer))
  (`|ExecutionSequence`
    (:`then_0`
      ;[1 0.9213 0] Enable / Disable input
      (set `self.CanOpen2?` false)
      (cast `/Game/ThirdPerson/Blueprints/BP_ThirdPersonCharacter` OtherActor)
      (`self.DisableInput` (`GameplayStatics.GetPlayerController` 0)))
    (:`then_1`
      (set `self.CanSee?` false)
      (`SceneComponent.SetVisibility` (`self.Widget`) false false))))

(event `self.ReceiveTick`
  (params (DeltaSeconds :type "Float (single-precision)")))

(fn `UserConstructionScript`)