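; BP_Digicode is a keypad actor, filed under a Level 1 door, that shows a code-entry widget while something is inside its box trigger.
; Overlap begin creates the WD_Digicode widget, shows the mouse cursor and sets UiIsActive on the player's BP_ThirdPersonCharacter; overlap end reverses this.
; On BeginPlay it stores a random four-digit code in that character's CodeCorrect variable, with no check on which actor overlaps.
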(event `self.Box.OnComponentBeginOverlap`
  (params (OverlappedComponent :type "PrimitiveComponent Object Reference") (OtherActor :type "Actor Object Reference") (OtherComp :type "PrimitiveComponent Object Reference") (OtherBodyIndex :type Integer) (bFromSweep :type Boolean) (SweepResult :type "HitResult Structure (by ref)"))
  (bind _returnvalue (`|CreateWidget` "/Game/UI/Digicode/Level1/WD_Digicode.WD_Digicode_C" null null))
  (bind _output_get (set `self.WD_Digicode_Ref` _returnvalue))
  (`UserWidget.AddToViewport` _output_get 0)
  (set `PlayerController.bShowMouseCursor` true (`GameplayStatics.GetPlayerController` 0))
  (bind _asbp_third_person_character (cast `/Game/ThirdPerson/Blueprints/BP_ThirdPersonCharacter` (`GameplayStatics.GetPlayerPawn` 0)))
  (set `/Game/ThirdPerson/Blueprints/BP_ThirdPersonCharacter.UiIsActive` true _asbp_third_person_character))

(event `self.Box.OnComponentEndOverlap`
  (params (OverlappedComponent :type "PrimitiveComponent Object Reference") (OtherActor :type "Actor Object Reference") (OtherComp :type "PrimitiveComponent Object Reference") (OtherBodyIndex :type Integer))
  (`Widget.RemoveFromParent` (`self.WD_Digicode_Ref`))
  (set `PlayerController.bShowMouseCursor` false (`GameplayStatics.GetPlayerController` 0))
  (set `/Game/ThirdPerson/Blueprints/BP_ThirdPersonCharacter.UiIsActive` false (stale `self.Box.OnComponentBeginOverlap` _asbp_third_person_character)))

(event `self.ReceiveBeginPlay`
  (bind _asbp_third_person_character (cast `/Game/ThirdPerson/Blueprints/BP_ThirdPersonCharacter` (`GameplayStatics.GetPlayerCharacter` 0)))
  (set `/Game/ThirdPerson/Blueprints/BP_ThirdPersonCharacter.CodeCorrect` (`KismetMathLibrary.RandomIntegerInRange` 1000 9999) _asbp_third_person_character))

(fn `UserConstructionScript`)