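; BP_Door is an interactive hinged door that the player opens and closes with the Interact input.
; A box trigger enables input while the third-person character overlaps it and disables it when they leave.
; Interact plays an open or close effect and runs a Timeline forward or in reverse, offsetting the mesh's yaw from its starting rotation.
; The closed state is derived from the current Timeline rotation.
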(event `self.ReceiveBeginPlay`
  ;[0 0.05647 1] Init Rotation
  (set `self.RotationDepart` (`SceneComponent.RelativeRotation` (`self.Porte`))))

(event `InputAction|Interact`
  (params (Key :type "Key Structure"))
  ;[0.02595 1 0] Open / Close Door
  (:`Pressed`
    (if (`self.close_Door`)
      (`AudioComponent.Play` (`self.OpenDoor`) 0.0)
      (bind (_direction _rotation) (`Timeline|Timeline` :!label _label)
        (:`Update`
          (`SceneComponent.K2_SetRelativeRotation` (`self.Porte`) (`KismetMathLibrary.MakeRotator` (.roll (`self.RotationDepart`)) (.pitch (`self.RotationDepart`)) (+ _rotation (.yaw (`self.RotationDepart`)))) false false)
          (set `self.close_Door` (< _rotation 1.0))))
      (else
        (`AudioComponent.Play` (`self.CloseDoor`) 0.0)
        (goto _label :!via `Reverse`)))))

(event `self.Box.OnComponentBeginOverlap`
  (params (OverlappedComponent :type "PrimitiveComponent Object Reference") (OtherActor :type "Actor Object Reference") (OtherComp :type "PrimitiveComponent Object Reference") (OtherBodyIndex :type Integer) (bFromSweep :type Boolean) (SweepResult :type "HitResult Structure (by ref)"))
  ;[1 0.9213 0] Enable / Disable input
  (cast `/Game/ThirdPerson/Blueprints/BP_ThirdPersonCharacter` (`GameplayStatics.GetPlayerCharacter` 0))
  (cast `/Game/ThirdPerson/Blueprints/BP_ThirdPersonCharacter` OtherActor)
  (`self.EnableInput` (`GameplayStatics.GetPlayerController` 0)))

(event `self.Box.OnComponentEndOverlap`
  (params (OverlappedComponent :type "PrimitiveComponent Object Reference") (OtherActor :type "Actor Object Reference") (OtherComp :type "PrimitiveComponent Object Reference") (OtherBodyIndex :type Integer))
  ;[1 0.9213 0] Enable / Disable input
  (cast `/Game/ThirdPerson/Blueprints/BP_ThirdPersonCharacter` OtherActor)
  (`self.DisableInput` (`GameplayStatics.GetPlayerController` 0)))

(fn `UserConstructionScript`)