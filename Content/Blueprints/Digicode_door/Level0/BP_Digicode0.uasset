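; Level 0 digicode actor that opens a keypad widget when the third-person character enters its box while CanActive is set.
; Overlap begin shows the mouse cursor and flags the character's UI as active; overlap end reverts both and removes the widget through WDDigicodeRef, which is not assigned here.
; BeginPlay stores a random four-digit correct code on the character, then briefly shows an "elevator unlocked" message (in French) on the help widget.
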(event `self.Box.OnComponentBeginOverlap`
  (params (OverlappedComponent :type "PrimitiveComponent Object Reference") (OtherActor :type "Actor Object Reference") (OtherComp :type "PrimitiveComponent Object Reference") (OtherBodyIndex :type Integer) (bFromSweep :type Boolean) (SweepResult :type "HitResult Structure (by ref)"))
  (cast `/Game/ThirdPerson/Blueprints/BP_ThirdPersonCharacter` OtherActor)
  (if (`self.CanActive`)
    (bind _returnvalue (`|CreateWidget` "/Game/UI/Digicode/Level0/WD_Digicode0.WD_Digicode0_C" null null))
    (`UserWidget.AddToViewport` _returnvalue 0)
    (set `PlayerController.bShowMouseCursor` true (`GameplayStatics.GetPlayerController` 0))
    (bind _asbp_third_person_character (cast `/Game/ThirdPerson/Blueprints/BP_ThirdPersonCharacter` (`GameplayStatics.GetPlayerPawn` 0)))
    (set `/Game/ThirdPerson/Blueprints/BP_ThirdPersonCharacter.UiIsActive` true _asbp_third_person_character)))

(event `self.Box.OnComponentEndOverlap`
  (params (OverlappedComponent :type "PrimitiveComponent Object Reference") (OtherActor :type "Actor Object Reference") (OtherComp :type "PrimitiveComponent Object Reference") (OtherBodyIndex :type Integer))
  (cast `/Game/ThirdPerson/Blueprints/BP_ThirdPersonCharacter` OtherActor)
  (if (`self.CanActive`)
    (`Widget.RemoveFromParent` (`self.WD_Digicode_Ref`))
    (set `PlayerController.bShowMouseCursor` false (`GameplayStatics.GetPlayerController` 0))
    (set `/Game/ThirdPerson/Blueprints/BP_ThirdPersonCharacter.UiIsActive` false (stale `self.Box.OnComponentBeginOverlap` _asbp_third_person_character))))

(event `self.ReceiveBeginPlay`
  (bind _asbp_third_person_character (cast `/Game/ThirdPerson/Blueprints/BP_ThirdPersonCharacter` (`GameplayStatics.GetPlayerCharacter` 0)))
  (set `/Game/ThirdPerson/Blueprints/BP_ThirdPersonCharacter.CodeCorrect` (`KismetMathLibrary.RandomIntegerInRange` 1000 9999) _asbp_third_person_character)
  (`KismetSystemLibrary.Delay` 0.5)
  (bind _foundwidgets (`WidgetBlueprintLibrary.GetAllWidgetsOfClass` "/Game/UI/WD_Aide.WD_Aide_C"))
  (bind _texteaide1 (`/Game/UI/WD_Aide.TexteAide1` (`|GetArrayItem` _foundwidgets)))
  (`TextBlock.SetText` _texteaide1 "ASCENCEUR DÉVERROUILLÉ")
  (`Widget.SetVisibility` _texteaide1 "Visible")
  (`KismetSystemLibrary.Delay` 3.0)
  (`Widget.SetVisibility` _texteaide1 "Hidden"))

(fn `UserConstructionScript`)