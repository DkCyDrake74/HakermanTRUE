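; BP_Digicode2 is a keypad trigger in the Level3 digicode door setup that opens a code-entry widget.
; On BeginPlay it clears CodeTrue and stores a random four-digit CodeCorrect on BP_ThirdPersonCharacter, so the code state lives on the player.
; Box overlap adds WD_Digicode3, shows the mouse cursor and sets UiIsActive; end overlap reverses this.
; The overlapping actor is not checked.
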(event `self.Box.OnComponentBeginOverlap`
  (params (OverlappedComponent :type "PrimitiveComponent Object Reference") (OtherActor :type "Actor Object Reference") (OtherComp :type "PrimitiveComponent Object Reference") (OtherBodyIndex :type Integer) (bFromSweep :type Boolean) (SweepResult :type "HitResult Structure (by ref)"))
  ;[0 0.1663 1] Display WD Digicode
  (bind _returnvalue (`|CreateWidget` "/Game/UI/Digicode/level3/WD_Digicode3.WD_Digicode3_C" null null))
  (`UserWidget.AddToViewport` _returnvalue 0)
  (set `PlayerController.bShowMouseCursor` true (`GameplayStatics.GetPlayerController` 0))
  (bind _asbp_third_person_character (cast `/Game/ThirdPerson/Blueprints/BP_ThirdPersonCharacter` (`GameplayStatics.GetPlayerPawn` 0)))
  (set `/Game/ThirdPerson/Blueprints/BP_ThirdPersonCharacter.UiIsActive` true _asbp_third_person_character))

(event `self.Box.OnComponentEndOverlap`
  (params (OverlappedComponent :type "PrimitiveComponent Object Reference") (OtherActor :type "Actor Object Reference") (OtherComp :type "PrimitiveComponent Object Reference") (OtherBodyIndex :type Integer))
  ;[0 0.1663 1] Display WD Digicode
  (`Widget.RemoveFromParent` (stale `self.Box.OnComponentBeginOverlap` _returnvalue))
  (set `PlayerController.bShowMouseCursor` false (`GameplayStatics.GetPlayerController` 0))
  (set `/Game/ThirdPerson/Blueprints/BP_ThirdPersonCharacter.UiIsActive` false (stale `self.Box.OnComponentBeginOverlap` _asbp_third_person_character)))

(event `self.ReceiveBeginPlay`
  (`|ExecutionSequence`
    (:`then_0`
      ;[0.4531 0 0.01614] Reset Digicode
      (bind _asbp_third_person_character (cast `/Game/ThirdPerson/Blueprints/BP_ThirdPersonCharacter` (`GameplayStatics.GetPlayerCharacter` 0)))
      (set `/Game/ThirdPerson/Blueprints/BP_ThirdPersonCharacter.CodeTrue` false _asbp_third_person_character))
    (:`then_1`
      ;[0.01499 1 0] Set Random Code
      (bind _asbp_third_person_character_2 (cast `/Game/ThirdPerson/Blueprints/BP_ThirdPersonCharacter` (`GameplayStatics.GetPlayerCharacter` 0)))
      (set `/Game/ThirdPerson/Blueprints/BP_ThirdPersonCharacter.CodeCorrect` (`KismetMathLibrary.RandomIntegerInRange` 1000 9999) _asbp_third_person_character_2))))

(fn `UserConstructionScript`)