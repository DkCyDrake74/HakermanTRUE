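; Sliding wall elevator door for Level 3 that opens or shuts by moving along world X once its Binary2IsOK flag is true.
; BeginPlay stores the start position, then Tick adds Speed to X each frame, without delta-time scaling.
; After at least 200 units of travel it sets Close, which stops the movement for good.
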(event `self.ReceiveBeginPlay`
  (set `self.InitPos` (`self.K2_GetActorLocation`)))

(event `self.ReceiveTick`
  (params (DeltaSeconds :type "Float (single-precision)"))
  (bind _returnvalue_x (`KismetMathLibrary.BreakVector` (`self.K2_GetActorLocation`)))
  (bind (_returnvalue_x_2 _returnvalue_y _returnvalue_z) (`KismetMathLibrary.BreakVector` (`self.K2_GetActorLocation`)))
  (bind _initpos_x (`KismetMathLibrary.BreakVector` (`self.InitPos`)))
  (if (`self.Binary2IsOK`)
    (if (not (`self.Close`))
      (`self.K2_SetActorLocation` (`KismetMathLibrary.MakeVector` (+ _returnvalue_x_2 (`self.Speed`)) _returnvalue_y _returnvalue_z))
      (if (<= (+ _initpos_x 200.0) _returnvalue_x)
        (set `self.Close` true)))))

(fn `UserConstructionScript`)