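; Level 3 drone that, once StartDrone is true, flies a scripted route through five waypoint actors with yaw turns between legs.
; BeginPlay caches waypoint locations, and Tick walks nested boolean flags, each set by a tolerance check on position or rotation.
; Movement uses fixed per-frame steps, applied again by failed checks, so speed is frame-rate dependent.
; At the last point it waits briefly, blends the view to BP_Camera_3_1 and destroys itself.
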(event `RotationDroite`
  (bind (_returnvalue_roll _returnvalue_pitch _returnvalue_yaw) (`KismetMathLibrary.BreakRotator` (`self.K2_GetActorRotation`)))
  ;[0.2969 0.2969 0.2969] Mechanics Rotation
  ;;[1 0.9496 0] Rotation Droite
  (`self.K2_SetActorRotation` (`KismetMathLibrary.MakeRotator` _returnvalue_roll _returnvalue_pitch (+ _returnvalue_yaw (`self.RotationSpeed`)))))

(event `MoveToWaypoints4`
  (bind (_returnvalue_x _returnvalue_y) (`KismetMathLibrary.BreakVector` (`self.K2_GetActorLocation`)))
  ;[0.3021 0.3021 0.3021] Pos 4
  ;;[0 0.136 1] Move To Pos 4
  (bind _returnvalue (`GameplayStatics.GetActorOfClass` "/Game/Blueprints/Drone/Waypoints/Waypoints_Drone4.Waypoints_Drone4_C"))
  (bind (_returnvalue_x_2 _returnvalue_y_2 _returnvalue_z) (`KismetMathLibrary.BreakVector` (`self.K2_GetActorLocation` _returnvalue)))
  (`self.K2_SetActorLocation` (`KismetMathLibrary.MakeVector` _returnvalue_x_2 (+ _returnvalue_y (`self.SpeedFront`)) _returnvalue_z)))

(event `MoveToWaypoints3`
  (bind _returnvalue_x (`KismetMathLibrary.BreakVector` (`self.K2_GetActorLocation`)))
  ;[0.3125 0.3125 0.3125] Pos3
  ;;[0 0.08885 1] Move To Pos 3
  (bind _returnvalue (`GameplayStatics.GetActorOfClass` "/Game/Blueprints/Drone/Waypoints/Waypoints_Drone3.Waypoints_Drone3_C"))
  (bind (_returnvalue_x_2 _returnvalue_y _returnvalue_z) (`KismetMathLibrary.BreakVector` (`self.K2_GetActorLocation` _returnvalue)))
  (`self.K2_SetActorLocation` (`KismetMathLibrary.MakeVector` (+ _returnvalue_x (`self.SpeedFront`)) _returnvalue_y _returnvalue_z)))

(event `VerifRotation`
  ;[0.2969 0.2969 0.2969] Mechanics Rotation
  ;;[1 0.02616 0] Verif Rotation
  (if (== (`self.DroneRotation`) (struct :`Yaw` 90.0))
    (set `self.FullRotation` true)
    (else
      (`self.RotationDroite`))))

(event `VerifIsOnPoint3`
  ;[0.3125 0.3125 0.3125] Pos3
  ;;[1 0.01661 0] Verif pos 3
  (if (== (`self.TargetPoint_3`) (`self.DronePosition`) :`ErrorTolerance` 20.0)
    (set `self.IsOnPoint_3` true)
    (else
      (`self.MoveToWaypoints3`))))

(event `VerifisOnPoints4`
  ;[0.3021 0.3021 0.3021] Pos 4
  ;;[1 0 0] Verif Pos 4
  (if (== (`self.TargetPoint_4`) (`self.DronePosition`) :`ErrorTolerance` 20.0)
    (set `self.IsOnPoint_4` true)
    (else
      (`self.MoveToWaypoints4`))))

(event `self.ReceiveTick`
  (params (DeltaSeconds :type "Float (single-precision)"))
  ;[0.06192 1 0] Verif per frame
  (set `self.DroneRotation` (`self.K2_GetActorRotation`))
  (set `self.DronePosition` (`self.K2_GetActorLocation`))
  (if (`self.StartDrone`)
    (if (`self.IsOnPoint_0`)
      (if (`self.IsOnPoint_1`)
        (if (`self.FullRotation`)
          (if (`self.IsOnPoint_2`)
            (if (`self.FullRotation1`)
              (if (`self.IsOnPoint_3`)
                (if (`self.FullRotation2`)
                  (if (`self.IsOnPoint_4`)
                    (`KismetSystemLibrary.Delay` 1.0)
                    (bind _returnvalue (`GameplayStatics.GetActorOfClass` "/Game/Blueprints/Camera/Camera/Level3/Camera_Level_3/BP_Camera_3_1.BP_Camera_3_1_C"))
                    (`PlayerController.SetViewTargetWithBlend` (`GameplayStatics.GetPlayerController` 0) _returnvalue 0.0 "VTBlend_Linear" 0.0 false)
                    (`self.K2_DestroyActor`)
                    (else
                      (`self.MoveToWaypoints4`)
                      (`self.VerifisOnPoints4`)))
                  (else
                    (`self.RotationDroite`)
                    (`self.VerifRotation3`)))
                (else
                  (`self.MoveToWaypoints3`)
                  (`self.VerifIsOnPoint3`)))
              (else
                (`self.RotationDroite`)
                (`self.VerifRotation2`)))
            (else
              (`self.MoveToWaypoints2`)
              (`self.VerifIsOnPoint2`)))
          (else
            (`self.RotationDroite`)
            (`self.VerifRotation`)))
        (else
          (`self.MoveToWaypoints1`)
          (`self.VerifIsOnPoint`)))
      (else
        (`self.MoveToStartPos`)
        (`self.VerifStartPos`)))))

(event `VerifRotation2`
  ;[0.2969 0.2969 0.2969] Mechanics Rotation
  ;;[1 0.05729 0.05729] verif Rotation 2
  (if (== (`self.DroneRotation`) (struct :`Yaw` 179.0))
    (set `self.FullRotation1` true)
    (else
      (`self.RotationDroite`))))

(event `MoveToWaypoints2`
  (bind (_returnvalue_x _returnvalue_y) (`KismetMathLibrary.BreakVector` (`self.K2_GetActorLocation`)))
  ;[0.3438 0.3438 0.3438] Pos 2
  ;;[0 0.05164 1] Move to Pos 2
  (bind _returnvalue (`GameplayStatics.GetActorOfClass` "/Game/Blueprints/Drone/Waypoints/Waypoints_Drone2.Waypoints_Drone2_C"))
  (bind (_returnvalue_x_2 _returnvalue_y_2 _returnvalue_z) (`KismetMathLibrary.BreakVector` (`self.K2_GetActorLocation` _returnvalue)))
  (`self.K2_SetActorLocation` (`KismetMathLibrary.MakeVector` _returnvalue_x_2 (+ _returnvalue_y (`self.SpeedBack`)) _returnvalue_z)))

(event `MoveToWaypoints1`
  (bind _returnvalue_x (`KismetMathLibrary.BreakVector` (`self.K2_GetActorLocation`)))
  ;[0.2938 0.2969 0.2907] Pos 1
  ;;[0 0.05776 1] Move To Pos 1
  (bind _returnvalue (`GameplayStatics.GetActorOfClass` "/Game/Blueprints/Drone/Waypoints/Waypoints_Drone1.Waypoints_Drone1_C"))
  (bind (_returnvalue_x_2 _returnvalue_y _returnvalue_z) (`KismetMathLibrary.BreakVector` (`self.K2_GetActorLocation` _returnvalue)))
  (`self.K2_SetActorLocation` (`KismetMathLibrary.MakeVector` (+ _returnvalue_x (`self.SpeedUp`)) _returnvalue_y _returnvalue_z)))

(event `VerifRotation3`
  ;[0.2969 0.2969 0.2969] Mechanics Rotation
  ;;[1 0 0] Verif rotation 2
  (if (== (`self.DroneRotation`) (struct :`Yaw` -90.0) :`ErrorTolerance` 2.0)
    (set `self.FullRotation2` true)
    (else
      (`self.RotationDroite`))))

(event `VerifIsOnPoint2`
  ;[0.3438 0.3438 0.3438] Pos 2
  ;;[1 0.00687 0] Verif is on pos 2
  (if (== (`self.TargetPoint_2`) (`self.DronePosition`) :`ErrorTolerance` 20.0)
    (set `self.IsOnPoint_2` true)
    (else
      (`self.MoveToWaypoints2`))))

(event `VerifIsOnPoint`
  ;[0.2938 0.2969 0.2907] Pos 1
  ;;[1 0 0.006241] Check if drone is on pos
  (if (== (`self.TargetPoint_1`) (`self.DronePosition`) :`ErrorTolerance` 20.0)
    (set `self.IsOnPoint_1` true)
    (else
      (`self.MoveToWaypoints1`))))

(event `MoveToStartPos`
  (bind (_returnvalue_x _returnvalue_y _returnvalue_z) (`KismetMathLibrary.BreakVector` (`self.K2_GetActorLocation`)))
  ;[0 0.1984 1] Move to start position
  (bind _returnvalue (`GameplayStatics.GetActorOfClass` "/Game/Blueprints/Drone/Waypoints/Waypoints_Drone.Waypoints_Drone_C"))
  (bind (_returnvalue_x_2 _returnvalue_y_2) (`KismetMathLibrary.BreakVector` (`self.K2_GetActorLocation` _returnvalue)))
  (`self.K2_SetActorLocation` (`KismetMathLibrary.MakeVector` _returnvalue_x_2 _returnvalue_y_2 (+ _returnvalue_z (`self.SpeedUp`)))))

(event `self.ReceiveBeginPlay`
  ;[0.008477 1 0] Set target pos
  (`|ExecutionSequence`
    (:`then_0`
      (bind _returnvalue (`GameplayStatics.GetActorOfClass` "/Game/Blueprints/Drone/Waypoints/Waypoints_Drone.Waypoints_Drone_C"))
      (bind _output_get (set `self.TargetPoint` (`self.K2_GetActorLocation` _returnvalue))))
    (:`then_1`
      (bind _returnvalue_2 (`GameplayStatics.GetActorOfClass` "/Game/Blueprints/Drone/Waypoints/Waypoints_Drone1.Waypoints_Drone1_C"))
      (set `self.TargetPoint_1` (`self.K2_GetActorLocation` _returnvalue_2)))
    (:`then_2`
      (bind _returnvalue_3 (`GameplayStatics.GetActorOfClass` "/Game/Blueprints/Drone/Waypoints/Waypoints_Drone2.Waypoints_Drone2_C"))
      (set `self.TargetPoint_2` (`self.K2_GetActorLocation` _returnvalue_3)))
    (:`then_3`
      (bind _returnvalue_4 (`GameplayStatics.GetActorOfClass` "/Game/Blueprints/Drone/Waypoints/Waypoints_Drone3.Waypoints_Drone3_C"))
      (set `self.TargetPoint_3` (`self.K2_GetActorLocation` _returnvalue_4)))
    (:`then_4`
      (bind _returnvalue_5 (`GameplayStatics.GetActorOfClass` "/Game/Blueprints/Drone/Waypoints/Waypoints_Drone4.Waypoints_Drone4_C"))
      (set `self.TargetPoint_4` (`self.K2_GetActorLocation` _returnvalue_5)))))

(event `VerifStartPos`
  ;[0.4583 0.02083 0] Verif Start Pos
  (if (== (stale `self.ReceiveBeginPlay` _output_get) (`self.DronePosition`) :`ErrorTolerance` 20.0)
    (set `self.IsOnPoint_0` true)
    (else
      (`self.MoveToStartPos`))))

(fn `UserConstructionScript`)