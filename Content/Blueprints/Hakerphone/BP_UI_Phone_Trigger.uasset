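; Trigger actor that manages the phone UI and a main widget through input and a Box volume.
; On BeginPlay it adds WD_Main to the viewport, and any overlap with the Box removes it.
; The OpenPhone input alternates through a FlipFlop between showing WD_Phone with the mouse cursor and clearing all widgets with the cursor hidden.
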(event `InputAction|OpenPhone`
  (params (Key :type "Key Structure"))
  ;[1 1 1] Activer / Désactiver le téléphone
  (:`Pressed`
    (bind _returnvalue (`|CreateWidget` "/Game/UI/UI_Phone/WD_Phone.WD_Phone_C"))
    (`/Engine/EditorBlueprintResources/StandardMacros.FlipFlop`
      (:`A`
        (bind _output_get (set `self.WD_Phone_Ref` _returnvalue))
        (`UserWidget.AddToViewport` _output_get 0)
        (set `PlayerController.bShowMouseCursor` true (`GameplayStatics.GetPlayerController` 0)))
      (:`B`
        (`WidgetLayoutLibrary.RemoveAllWidgets`)
        (set `PlayerController.bShowMouseCursor` false (`GameplayStatics.GetPlayerController` 0))))))

(event `self.ReceiveBeginPlay`
  ;[1 1 1] Create widget Ref
  (bind _returnvalue (`|CreateWidget` "/Game/UI/WD_Main.WD_Main_C"))
  (bind _output_get (set `self.WD_Main_Ref` _returnvalue))
  (`UserWidget.AddToViewport` _output_get 0))

(event `self.Box.OnComponentBeginOverlap`
  (params (OverlappedComponent :type "PrimitiveComponent Object Reference") (OtherActor :type "Actor Object Reference") (OtherComp :type "PrimitiveComponent Object Reference") (OtherBodyIndex :type Integer) (bFromSweep :type Boolean) (SweepResult :type "HitResult Structure (by ref)"))
  ;[1 1 1] Create widget Ref
  (`Widget.RemoveFromParent` (stale `self.ReceiveBeginPlay` _output_get)))

(fn `UserConstructionScript`)