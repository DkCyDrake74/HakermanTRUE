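; BP_Switch_Light is an interactable light switch that briefly blacks out tagged ceiling lights as a diversion for Level 2 guards.
; On Tick, player proximity toggles input and the switch's custom-depth highlight, and enables tagged post-process volumes, which are never disabled again.
; Interact zeroes the lights' intensity, restores it after a five-second Delay placed inside the loop, and calls LightEvent on every BP_AI_gardes_Level_2 guard.
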(event `InputAction|Interact`
  (params (Key :type "Key Structure"))
  (:`Pressed`
    (`|ExecutionSequence`
      (:`then_0`
        (bind _outactors (`GameplayStatics.GetAllActorsOfClassWithTag` "/Game/StarterContent/Blueprints/Blueprint_CeilingLight.Blueprint_CeilingLight_C" "Light"))
        (for _array_element _outactors
          (`LightComponent.SetIntensity` (`/Game/StarterContent/Blueprints/Blueprint_CeilingLight.PointLight1` _array_element) 0.0)
          (`KismetSystemLibrary.Delay` 5.0)
          (bind _outactors_2 (`GameplayStatics.GetAllActorsOfClassWithTag` "/Game/StarterContent/Blueprints/Blueprint_CeilingLight.Blueprint_CeilingLight_C" "Light"))
          (for _array_element_2 _outactors_2
            (`LightComponent.SetIntensity` (`/Game/StarterContent/Blueprints/Blueprint_CeilingLight.PointLight1` _array_element_2) 1700.0))))
      (:`then_1`
        (bind _outactors_3 (`GameplayStatics.GetAllActorsOfClass` "/Game/AI/Gardes/Level2/GardesRandom/BP_AI_gardes_Level_2.BP_AI_gardes_Level_2_C"))
        (for _array_element_3 _outactors_3
          (`/Game/AI/Gardes/Level2/GardesRandom/BP_AI_gardes_Level_2.LightEvent` _array_element_3))))))

(event `self.ReceiveTick`
  (params (DeltaSeconds :type "Float (single-precision)"))
  (bind _returnvalue (`GameplayStatics.GetPlayerController` 0))
  (bind _sm_lightswitch_01 (`self.SM_Lightswitch_01`))
  (if (<= (`KismetMathLibrary.Vector_Distance` (`self.K2_GetActorLocation` (`GameplayStatics.GetPlayerCharacter` 0)) (`self.K2_GetActorLocation`)) (`self.MaxDistance`))
    (`self.EnableInput` _returnvalue)
    (`PrimitiveComponent.SetRenderCustomDepth` _sm_lightswitch_01 true)
    (bind _outactors (`GameplayStatics.GetAllActorsOfClassWithTag` "/Script/Engine.PostProcessVolume" "PP"))
    (for _array_element _outactors
      (set `PostProcessVolume.bEnabled` true _array_element))
    (else
      (`self.DisableInput` _returnvalue)
      (`PrimitiveComponent.SetRenderCustomDepth` _sm_lightswitch_01 false)
      (bind _outactors_2 (`GameplayStatics.GetAllActorsOfClassWithTag` "/Script/Engine.PostProcessVolume" "PP"))
      (for _array_element_2 _outactors_2
        _))))

(fn `UserConstructionScript`)