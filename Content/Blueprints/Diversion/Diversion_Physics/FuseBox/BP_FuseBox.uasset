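; BP_FuseBox is an interactable fuse box that serves as a diversion for the Level 2 guards.
; Pressing Interact sets FuseBoxIsTrigger on the first BP_AI_gardes_Level_2 found, then activates spark and smoke effects.
; Box overlaps toggle CanUse, though the Interact event never checks it.
; BeginPlay caches the actor's location.
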(event `self.ReceiveBeginPlay`
  (set `self.Location` (`self.K2_GetActorLocation`)))

(event `InputAction|Interact`
  (params (Key :type "Key Structure"))
  (:`Pressed`
    (`|ExecutionSequence`
      (:`then_0`
        (bind _outactors (`GameplayStatics.GetAllActorsOfClass` "/Game/AI/Gardes/Level2/GardesRandom/BP_AI_gardes_Level_2.BP_AI_gardes_Level_2_C"))
        (set `/Game/AI/Gardes/Level2/GardesRandom/BP_AI_gardes_Level_2.FuseBoxIsTrigger` true (`|GetArrayItem` _outactors)))
      (:`then_1`
        (`ActorComponent.Activate` (`self.Spark`) false)
        (`ActorComponent.Activate` (`self.P_Smoke_A`) false)))))

(event `self.Box.OnComponentBeginOverlap`
  (params (OverlappedComponent :type "PrimitiveComponent Object Reference") (OtherActor :type "Actor Object Reference") (OtherComp :type "PrimitiveComponent Object Reference") (OtherBodyIndex :type Integer) (bFromSweep :type Boolean) (SweepResult :type "HitResult Structure (by ref)"))
  (set `self.CanUse?` true))

(event `self.Box.OnComponentEndOverlap`
  (params (OverlappedComponent :type "PrimitiveComponent Object Reference") (OtherActor :type "Actor Object Reference") (OtherComp :type "PrimitiveComponent Object Reference") (OtherBodyIndex :type Integer))
  (set `self.CanUse?` false))

(fn `UserConstructionScript`)