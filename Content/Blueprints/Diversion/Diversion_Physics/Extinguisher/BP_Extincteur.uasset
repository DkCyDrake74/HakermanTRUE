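; BP_Extincteur is a one-shot extinguisher diversion that the player triggers to alert Level 2 guard AI.
; Tick checks player distance against MaxDistance, toggling CanInteract and the actor's input.
; Interact plays audio and sets ExtinguisherIsTrigger on every BP_AI_gardes_Level_2.
; A Delay inside that loop later stops the audio and clears the flag, but only on the loop's final element.
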(event `self.ReceiveTick`
  (params (DeltaSeconds :type "Float (single-precision)"))
  (bind _returnvalue (`GameplayStatics.GetPlayerController` 0))
  (if (<= (`KismetMathLibrary.Vector_Distance` (`self.K2_GetActorLocation` (`GameplayStatics.GetPlayerCharacter` 0)) (`self.K2_GetActorLocation`)) (`self.MaxDistance`))
    (set `self.CanInteract` true)
    (`self.EnableInput` _returnvalue)
    (else
      (set `self.CanInteract` false)
      (`self.DisableInput` _returnvalue))))

(event `self.ReceiveBeginPlay`
  (set `self.Location` (`self.K2_GetActorLocation`)))

(event `InputAction|Interact`
  (params (Key :type "Key Structure"))
  (:`Pressed`
    (if (`self.CanInteract`)
      (`/Engine/EditorBlueprintResources/StandardMacros.DoOnce` false
        (:`Completed`
          (`AudioComponent.Play` (`self.Audio`) 0.0)
          (bind _outactors (`GameplayStatics.GetAllActorsOfClass` "/Game/AI/Gardes/Level2/GardesRandom/BP_AI_gardes_Level_2.BP_AI_gardes_Level_2_C"))
          (for _array_element _outactors
            (set `/Game/AI/Gardes/Level2/GardesRandom/BP_AI_gardes_Level_2.ExtinguisherIsTrigger` true _array_element)
            (`KismetSystemLibrary.Delay` 10.0)
            (`AudioComponent.Stop` (`self.Audio`))
            (set `/Game/AI/Gardes/Level2/GardesRandom/BP_AI_gardes_Level_2.ExtinguisherIsTrigger` false _array_element)))))))

(fn `UserConstructionScript`)