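; BP_distributer is an interactable distributor that serves as a diversion for the level 2 guard AI.
; A box overlap toggles whether the Interact input is accepted, and BeginPlay stores the actor's location.
; Interacting sets DistributerIsTrigger on every BP_AI_gardes_Level_2.
; A Delay inside that loop precedes clearing the flag, so only the last guard is likely reset.
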(event `self.ReceiveBeginPlay`
  (set `self.DistributerLocation` (`self.K2_GetActorLocation`)))

(event `InputAction|Interact`
  (params (Key :type "Key Structure"))
  (:`Pressed`
    (if (`self.CanInteract?`)
      (bind _outactors (`GameplayStatics.GetAllActorsOfClass` "/Game/AI/Gardes/Level2/GardesRandom/BP_AI_gardes_Level_2.BP_AI_gardes_Level_2_C"))
      (for _array_element _outactors
        (set `/Game/AI/Gardes/Level2/GardesRandom/BP_AI_gardes_Level_2.DistributerIsTrigger` true _array_element)
        (`KismetSystemLibrary.Delay` 10.0)
        (set `/Game/AI/Gardes/Level2/GardesRandom/BP_AI_gardes_Level_2.DistributerIsTrigger` false _array_element)))))

(event `self.Box.OnComponentBeginOverlap`
  (params (OverlappedComponent :type "PrimitiveComponent Object Reference") (OtherActor :type "Actor Object Reference") (OtherComp :type "PrimitiveComponent Object Reference") (OtherBodyIndex :type Integer) (bFromSweep :type Boolean) (SweepResult :type "HitResult Structure (by ref)"))
  (set `self.CanInteract?` true))

(event `self.Box.OnComponentEndOverlap`
  (params (OverlappedComponent :type "PrimitiveComponent Object Reference") (OtherActor :type "Actor Object Reference") (OtherComp :type "PrimitiveComponent Object Reference") (OtherBodyIndex :type Integer))
  (set `self.CanInteract?` false))

(fn `UserConstructionScript`)