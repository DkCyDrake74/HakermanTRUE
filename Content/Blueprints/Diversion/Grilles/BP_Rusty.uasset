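; BP_Rusty is a grille that rises 120 units to open and drops back down to close, with an uneven motion.
; GridIsTrigger starts the rise and GridIsTrigger2 the descent, but neither is set to true within this Blueprint.
; Tick moves the actor by a random 1–3 units per frame without delta-time scaling, clearing each trigger once its height limit is reached.
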(event `self.ReceiveBeginPlay`
  (set `self.GridPosClose` (`self.K2_GetActorLocation`)))

(event `self.ReceiveTick`
  (params (DeltaSeconds :type "Float (single-precision)"))
  (bind (_returnvalue_x _returnvalue_y _returnvalue_z) (`KismetMathLibrary.BreakVector` (`self.K2_GetActorLocation`)))
  (bind (_returnvalue_x_2 _returnvalue_y_2 _returnvalue_z_2) (`KismetMathLibrary.BreakVector` (`self.K2_GetActorLocation`)))
  (bind (_returnvalue_x_3 _returnvalue_y_3 _returnvalue_z_3) (`KismetMathLibrary.BreakVector` (`self.K2_GetActorLocation`)))
  (bind (_returnvalue_x_4 _returnvalue_y_4 _returnvalue_z_4) (`KismetMathLibrary.BreakVector` (`self.K2_GetActorLocation`)))
  (bind (_gridposclose_x _gridposclose_y _gridposclose_z) (`KismetMathLibrary.BreakVector` (`self.GridPosClose`)))
  (bind (_gridposopen_x _gridposopen_y _gridposopen_z) (`KismetMathLibrary.BreakVector` (`self.GridPosOpen`)))
  (bind _returnvalue (+ _gridposclose_z 120.0))
  (if (and (`self.GridIsOpen?`) (`self.GridIsTrigger2?`))
    (if (`self.GridIsTrigger2?`)
      (`self.K2_SetActorLocation` (`KismetMathLibrary.MakeVector` _returnvalue_x_3 _returnvalue_y_3 (+ _returnvalue_z_3 (`KismetMathLibrary.RandomFloatInRange` -1.0 -3.0))))
      (if (<= _returnvalue_z_2 (- _gridposopen_z 120.0))
        (set `self.GridIsOpen?` false)
        (set `self.GridIsTrigger2?` false)))
    (elif (`self.GridIsTrigger?`)
      (`self.K2_SetActorLocation` (`KismetMathLibrary.MakeVector` _returnvalue_x_4 _returnvalue_y_4 (+ _returnvalue_z_4 (`KismetMathLibrary.RandomFloatInRange` 1.0 3.0))))
      (set `self.GridIsOpen?` true)
      (if (>= _returnvalue_z _returnvalue)
        (set `self.GridIsTrigger?` false)
        (set `self.GridPosOpen` (`KismetMathLibrary.MakeVector` _gridposclose_x _gridposclose_y _returnvalue))))))

(fn `UserConstructionScript`)