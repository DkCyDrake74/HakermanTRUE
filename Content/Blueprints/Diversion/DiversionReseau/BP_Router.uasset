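; BP_Router is a network-diversion prop, built from electric meter meshes, that signals when the player is close enough to hack.
; Every Tick it compares its distance to player 0 against MaxDistance and sets HackRange on BP_ThirdPersonCharacter accordingly.
; The same check toggles custom depth rendering on the meter's base and box meshes.
; HackRange is also written false when out of range, so multiple routers would overwrite each other's value.
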(event `self.ReceiveTick`
  (params (DeltaSeconds :type "Float (single-precision)"))
  (bind _sm_electricmeterset01base (`self.SM_ElectricMeterSet01Base`))
  (if (<= (`KismetMathLibrary.Vector_Distance` (`self.K2_GetActorLocation` (`GameplayStatics.GetPlayerCharacter` 0)) (`self.K2_GetActorLocation`)) (`self.MaxDistance`))
    (bind _asbp_third_person_character (cast `/Game/ThirdPerson/Blueprints/BP_ThirdPersonCharacter` (`GameplayStatics.GetPlayerCharacter` 0)))
    (set `/Game/ThirdPerson/Blueprints/BP_ThirdPersonCharacter.HackRange?` true _asbp_third_person_character)
    (`PrimitiveComponent.SetRenderCustomDepth` _sm_electricmeterset01base true)
    (`PrimitiveComponent.SetRenderCustomDepth` (`self.SM_ElectricMeterSet01Box`) true)
    (else
      (bind _asbp_third_person_character_2 (cast `/Game/ThirdPerson/Blueprints/BP_ThirdPersonCharacter` (`GameplayStatics.GetPlayerCharacter` 0)))
      (set `/Game/ThirdPerson/Blueprints/BP_ThirdPersonCharacter.HackRange?` false _asbp_third_person_character_2)
      (`PrimitiveComponent.SetRenderCustomDepth` _sm_electricmeterset01base false)
      (`PrimitiveComponent.SetRenderCustomDepth` (`self.SM_ElectricMeterSet01Box`) false))))

(fn `UserConstructionScript`)